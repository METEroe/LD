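; Enemy chess-piece pawn whose data table row sets its mesh on construction and selects its attack on BeginPlay.
; Queen, Bishop, Rook and Archer use timelines scaled by fire rate to spawn BP_EnemyBullet with effects and sound.
; Queen fires at random yaw, Bishop four ways diagonally, Rook and Archer along the arrow, while Knight moves in an L without shooting.
; AnyDamage reduces health and destroys the pawn at zero.
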(event Custom|Archer_Attack
  ;[1 1 1] Archer
  (Components|Timeline|SetPlayRate (Variables|Default|GetArcherTimeline) (Variables|Archer|GetArcher%20Fire%20Rate))
  (Timeline|ArcherTimeline Play
    (:Archer_Attack
      (CallFunction|ArcherFire (Variables|Default|GetArrow)))))

(event Custom|Queen%20Fire
  (params (Target :type Scene%20Component%20Object%20Reference))
  (bind _returnvalue (Transformation|GetWorldLocation Target))
  (bind _returnvalue_2 (Transformation|GetWorldTransform Target))
  ;[1 1 1] Queen
  (Niagara|SpawnSystematLocation 0 _returnvalue "0.000000,90.000000,0.000000")
  (Audio|PlaySoundatLocation 0 _returnvalue "0, 0, 0" 1.0 1.0 0.0 0 0 0 0)
  (Game|SpawnActorfromClass "/Game/Piece/BluePrints/BP_EnemyBullet.BP_EnemyBullet_C" (Math|Transform|MakeTransform (.location _returnvalue_2) (Math|Rotator|MakeRotator (.roll (.rotation _returnvalue_2)) (.pitch (.rotation _returnvalue_2)) (+ (.yaw (.rotation _returnvalue_2)) (* (Math|Random|RandomFloat) 3.6e+02))) (.scale _returnvalue_2)) "Undefined" "MultiplyWithRoot" 0 (Variables|Queen|GetQueen%20Initial%20Speed) (Variables|Queen|GetQueen%20Projectile%20Gravity%20Scale) (Variables|Queen|GetQueen%20In%20Lifespan) (Variables|Queen|GetQueen%20Damage) (Variables|Default|GetInstigator_0)))

(event Custom|PieceCheck
  (bind _piecescheck (Variables|Default|GetPiecesCheck))
  (bind _returnvalue (Utilities|GetDataTableRow (.datatable (.piecestable _piecescheck)) (.rowname (.piecestable _piecescheck)))
    (:then
      (switch name (.Name (Utilities|Struct|BreakPieceListStruct _returnvalue))
        (:Queen
          (CallFunction|QueenAttack))
        (:Bishop
          (CallFunction|BishopAttack))
        (:Knight
          (CallFunction|KnightAttack))
        (:Rook
          (CallFunction|RookAttack))
        (:Archer
          (CallFunction|ArcherAttack))))))

(event Custom|Knight_Attack
  (bind _capsule (Variables|Default|GetCapsule))
  (bind _capsule_2 (Variables|Default|GetCapsule))
  ;[1 1 1] Knight
  (bind _output_get (Variables|Default|SetStartLocation (Transformation|GetWorldLocation _capsule)))
  (Components|MoveComponentTo (Variables|Default|GetCapsule) (+ _output_get (* (Math|Vector|GetForwardVector _capsule) 300)) "0, 0, 0" false false 1.0 false)
  (bind _output_get_2 (Variables|Default|SetStartLocation (Transformation|GetWorldLocation _capsule_2)))
  (Components|MoveComponentTo (Variables|Default|GetCapsule) (+ _output_get_2 (* (Math|Vector|GetRightVector _capsule_2) 150)) "0, 0, 0" false false 1.0 false))

(event Custom|Bishop_Attack
  ;[1 1 1] Bishop
  (Components|Timeline|SetPlayRate (Variables|Default|GetBishopTimeline) (Variables|Bishop|GetBishop%20Fire%20Rate))
  (Timeline|BishopTimeline Play
    (:Bishop_Attack
      (CallFunction|BishopFire (Variables|Default|GetArrow)))))

(event Custom|Bishop_Fire
  (params (Target :type Scene%20Component%20Object%20Reference))
  (bind _returnvalue (Transformation|GetWorldLocation Target))
  ;[1 1 1] Bishop
  (Niagara|SpawnSystematLocation 0 _returnvalue "0.000000,90.000000,0.000000")
  (Audio|PlaySoundatLocation 0 _returnvalue "0, 0, 0" 1.0 1.0 0.0 0 0 0 0)
  (CallFunction|Four-wayDiagonalShooting Target (Variables|Bishop|GetBishop%20Initial%20Speed) (Variables|Bishop|GetBishop%20Projectile%20Gravity%20Scale) (Variables|Bishop|GetBishop%20In%20Lifespan) (Variables|Bishop|GetBishop%20Damage)))

(event Custom|Queen_Attack
  ;[1 1 1] Queen
  (Components|Timeline|SetPlayRate (Variables|Default|GetQueenTimeline) (Variables|Queen|GetQueen%20Fire%20Rate))
  (Timeline|QueenTimeline Play
    (:Queen_Attack
      (CallFunction|QueenFire (Variables|Default|GetArrow)))))

(event Custom|Rook_Attack
  ;[1 1 1] Rook
  (Components|Timeline|SetPlayRate (Variables|Default|GetRookTimeline) (Variables|Rook|GetRook%20Fire%20Rate))
  (Timeline|RookTimeline Play
    (:Rook_Attack
      (CallFunction|RookFire (Variables|Default|GetArrow)))))

(event Custom|Archer%20Fire
  (params (Target :type Scene%20Component%20Object%20Reference))
  (bind _returnvalue (Transformation|GetWorldLocation Target))
  ;[1 1 1] Archer
  (Niagara|SpawnSystematLocation 0 _returnvalue "0.000000,90.000000,0.000000")
  (Audio|PlaySoundatLocation 0 _returnvalue "0, 0, 0" 1.0 1.0 0.0 0 0 0 0)
  (Game|SpawnActorfromClass "/Game/Piece/BluePrints/BP_EnemyBullet.BP_EnemyBullet_C" (Transformation|GetWorldTransform Target) "Undefined" "MultiplyWithRoot" 0 (Variables|Archer|GetArcher%20Initial%20Speed) (Variables|Archer|GetArcher%20Projectile%20Gravity%20Scale) (Variables|Archer|GetArcher%20In%20Lifespan) (Variables|Archer|GetArcher%20Damage) 0))

(event Custom|Rook%20Fire
  (params (Target :type Scene%20Component%20Object%20Reference))
  (bind _returnvalue (Transformation|GetWorldLocation Target))
  ;[1 1 1] Rook
  (Niagara|SpawnSystematLocation 0 _returnvalue "0.000000,90.000000,0.000000")
  (Audio|PlaySoundatLocation 0 _returnvalue "0, 0, 0" 1.0 1.0 0.0 0 0 0 0)
  (Game|SpawnActorfromClass "/Game/Piece/BluePrints/BP_EnemyBullet.BP_EnemyBullet_C" (Transformation|GetWorldTransform Target) "Undefined" "MultiplyWithRoot" 0 (Variables|Rook|GetRook%20Initial%20Speed) (Variables|Rook|GetRook%20Projectile%20Gravity%20Scale) (Variables|Rook|GetRook%20In%20Lifespan) (Variables|Rook|GetRook%20Damage) 0))

(event Game|Damage|EventAnyDamage
  (params (Damage :type Float%20%28single-precision%29) (DamageType :type Damage%20Type%20Object%20Reference) (InstigatedBy :type Controller%20Object%20Reference) (DamageCauser :type Actor%20Object%20Reference))
  ;[1 1 1] Health
  (bind _output_get (Variables|Health|SetHealth (- (Variables|Health|GetHealth) Damage)))
  (if (<= _output_get 0.0)
    (Audio|PlaySoundatLocation 0 (Transformation|GetActorLocation) "0, 0, 0" 1.0 1.0 0.0 0 0 0 0)
    (Development|PrintString "Dead!")
    (Variables|Health|SetHealth 0.0)
    (Actor|DestroyActor)
    (elif (> (Variables|Health|GetHealth) (Variables|Health|GetMax_Health))
      (Variables|Health|SetHealth (Variables|Health|GetMax_Health)))))

(event EventBeginPlay
  (CallFunction|PieceCheck))

(fn ConstructionScript
  (bind _piecescheck (Variables|Default|GetPiecesCheck))
  (bind _returnvalue (Utilities|GetDataTableRow (.datatable (.piecestable _piecescheck)) (.rowname (.piecestable _piecescheck)))
    (:then
      (Components|SkeletalMesh|SetSkeletalMeshAsset (Variables|Default|GetSkeletalMesh) (.Mesh (Utilities|Struct|BreakPieceListStruct _returnvalue))))))

(fn Four-wayDiagonalShooting
  (params (Arrow :type Scene%20Component%20Object%20Reference) (Initial%20Speed :type Float%20%28single-precision%29) (Projectile%20Gravity%20Scale :type Float%20%28single-precision%29) (In%20Lifespan :type Float%20%28single-precision%29) (Base%20Damage :type Float%20%28single-precision%29))
  (bind _returnvalue (Transformation|GetWorldTransform Arrow))
  (Utilities|FlowControl|Sequence
    (:then_0
      (Game|SpawnActorfromClass "/Game/Piece/BluePrints/BP_EnemyBullet.BP_EnemyBullet_C" (Math|Transform|MakeTransform (.location _returnvalue) (Math|Rotator|MakeRotator (.roll (.rotation _returnvalue)) (.pitch (.rotation _returnvalue)) (- (.yaw (.rotation _returnvalue)) 45.0)) (.scale _returnvalue)) "Undefined" "MultiplyWithRoot" 0 Initial%20Speed Projectile%20Gravity%20Scale In%20Lifespan Base%20Damage 0))
    (:then_1
      (Game|SpawnActorfromClass "/Game/Piece/BluePrints/BP_EnemyBullet.BP_EnemyBullet_C" (Math|Transform|MakeTransform (.location _returnvalue) (Math|Rotator|MakeRotator (.roll (.rotation _returnvalue)) (.pitch (.rotation _returnvalue)) (+ (.yaw (.rotation _returnvalue)) 45.0)) (.scale _returnvalue)) "Undefined" "MultiplyWithRoot" 0 Initial%20Speed Projectile%20Gravity%20Scale In%20Lifespan Base%20Damage 0))
    (:then_2
      (Game|SpawnActorfromClass "/Game/Piece/BluePrints/BP_EnemyBullet.BP_EnemyBullet_C" (Math|Transform|MakeTransform (.location _returnvalue) (Math|Rotator|MakeRotator (.roll (.rotation _returnvalue)) (.pitch (.rotation _returnvalue)) (- (.yaw (.rotation _returnvalue)) 135.0)) (.scale _returnvalue)) "Undefined" "MultiplyWithRoot" 0 Initial%20Speed Projectile%20Gravity%20Scale In%20Lifespan Base%20Damage 0))
    (:then_3
      (Game|SpawnActorfromClass "/Game/Piece/BluePrints/BP_EnemyBullet.BP_EnemyBullet_C" (Math|Transform|MakeTransform (.location _returnvalue) (Math|Rotator|MakeRotator (.roll (.rotation _returnvalue)) (.pitch (.rotation _returnvalue)) (+ (.yaw (.rotation _returnvalue)) 135.0)) (.scale _returnvalue)) "Undefined" "MultiplyWithRoot" 0 Initial%20Speed Projectile%20Gravity%20Scale In%20Lifespan Base%20Damage 0))))