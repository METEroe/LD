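; Chess-piece pawn for both player and enemy factions that auto-attacks according to its piece type.
; Construction loads mesh and projectile stats from T_Chess and sets faction tags and targets.
; Players attack continuously; enemies advance until a forward trace finds a player, with a fire-rate-scaled Timeline triggering attacks.
; Most types fire bullet patterns, Knight moves in an L, and enemies reaching zero health notify the controller and are destroyed.
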(event Custom|Make%20decision
  (bind _capsule (Variables|Default|GetCapsule))
  (switch Utilities|FlowControl|Switch|SwitchonE_ChessType (Variables|CommonData|GetPawn%20Type)
    (:NewEnumerator6
      (if (Math|Random|RandomBool)
        (Transformation|SetWorldRotation _capsule "0.000000,45.000000,0.000000" false false)
        (Transformation|SetWorldLocation (Variables|Default|GetCapsule) (- (Transformation|GetWorldLocation (Variables|Default|GetCapsule)) (Math|Vector|MakeVector 0.0 (* (Variables|CommonData|GetEnemy%20Speed) (Utilities|Time|GetWorldDeltaSeconds)) 0.0)) false false)
        (else
          (Transformation|SetWorldRotation _capsule "0.000000,-45.000000,0.000000" false false)
          (Transformation|SetWorldLocation (Variables|Default|GetCapsule) (+ (Transformation|GetWorldLocation (Variables|Default|GetCapsule)) (Math|Vector|MakeVector 0.0 (* (Variables|CommonData|GetEnemy%20Speed) (Utilities|Time|GetWorldDeltaSeconds)) 0.0)) false false))))))

(event Custom|Attack
  (if (Variables|CommonData|GetIn%20Attack%20Range)
    (Timeline|Timeline Play
      (:Archer_Attack
        (CallFunction|AttackDispatch)))))

(event Custom|Update%20Player%20Rate)

(event Custom|Attack%20Dispatch
  (bind _arrow (Variables|Default|GetArrow))
  (bind _arrow_2 (Variables|Default|GetArrow))
  (bind _capsule (Variables|Default|GetCapsule))
  (bind _capsule_2 (Variables|Default|GetCapsule))
  (bind _arrow_3 (Variables|Default|GetArrow))
  (bind _arrow_4 (Variables|Default|GetArrow))
  (bind _returnvalue (Transformation|GetWorldLocation _arrow_2))
  (bind _returnvalue_2 (Transformation|GetWorldLocation _arrow))
  (bind _returnvalue_3 (Transformation|GetWorldLocation _arrow_3))
  (bind _returnvalue_4 (Transformation|GetWorldLocation _arrow_4))
  (switch Utilities|FlowControl|Switch|SwitchonE_ChessType (Variables|CommonData|GetPawn%20Type)
    (:NewEnumerator1
      (Niagara|SpawnSystematLocation 0 _returnvalue_2 "0.000000,90.000000,0.000000")
      (Audio|PlaySoundatLocation 0 _returnvalue_2 "0, 0, 0" 1.0 1.0 0.0 0 0 0 0)
      (Utilities|ForLoopwithDelay 0 3 0.2
        (:Loop%20Body
          (Transformation|AddRelativeRotation (Variables|Default|GetArrow) (Math|Rotator|MakeRotator 0.0 0.0 (Math|Random|RandomFloatinRange 0.0 3.6e+02)) false false)
          (CallFunction|FireBullet))))
    (:NewEnumerator5
      (bind _output_get (Variables|CommonData|SetSpawnLocation (Transformation|GetWorldLocation _capsule)))
      (Components|MoveComponentTo (Variables|Default|GetCapsule) (+ _output_get (* (Math|Vector|GetForwardVector _capsule) 300)) "0, 0, 0" false false 1.0 false)
      (bind _output_get_2 (Variables|CommonData|SetSpawnLocation (Transformation|GetWorldLocation _capsule_2)))
      (Components|MoveComponentTo (Variables|Default|GetCapsule) (+ _output_get_2 (* (Math|Vector|GetRightVector _capsule_2) 150)) "0, 0, 0" false false 1.0 false))
    (:NewEnumerator2
      (Niagara|SpawnSystematLocation 0 _returnvalue "0.000000,90.000000,0.000000")
      (Audio|PlaySoundatLocation 0 _returnvalue "0, 0, 0" 1.0 1.0 0.0 0 0 0 0)
      (bind _index (Utilities|ForLoopwithDelay 0 3 0.0)
        (:Loop%20Body
          (Transformation|SetRelativeRotation (Variables|Default|GetArrow) (Math|Rotator|MakeRotator 0.0 0.0 (Math|Conversions|ToFloat(Integer) (+ (* _index 90) 45))) false false)
          (CallFunction|FireBullet))))
    (:NewEnumerator3
      (Niagara|SpawnSystematLocation 0 _returnvalue_4 "0.000000,90.000000,0.000000")
      (Audio|PlaySoundatLocation 0 _returnvalue_4 "0, 0, 0" 1.0 1.0 0.0 0 0 0 0)
      (CallFunction|FireBullet))
    (:NewEnumerator4
      (Niagara|SpawnSystematLocation 0 _returnvalue_3 "0.000000,90.000000,0.000000")
      (Audio|PlaySoundatLocation 0 _returnvalue_3 "0, 0, 0" 1.0 1.0 0.0 0 0 0 0)
      (CallFunction|FireBullet))))

(event Custom|Fire%20Bullet
  (Game|SpawnActorfromClass "/Game/Piece/BluePrints/BP_Bullet.BP_Bullet_C" (Transformation|GetWorldTransform (Variables|Default|GetArrow)) "Undefined" "MultiplyWithRoot" 0 (Variables|Default|GetInitial%20Speed) (Variables|Default|GetProject%20Gravity%20Scale) (Variables|Default|GetLife%20Span) (Math|Float|Truncate (Variables|Default|GetDamage)) (Variables|CommonData|GetHit%20Target%20Actor) 0))

(event EventTick
  (params (DeltaSeconds :type Float%20%28single-precision%29))
  (bind _capsule (Variables|Default|GetCapsule))
  (bind _returnvalue (Transformation|GetWorldLocation _capsule))
  (CallFunction|MakeDecision)
  (CallFunction|Attack)
  (if (Variables|CommonData|GetIs%20Enemy)
    (Utilities|FlowControl|Sequence
      (:then_0
        (bind (_outhit _returnvalue_2) (Collision|LineTraceForObjects _returnvalue (+ _returnvalue (* (Math|Vector|GetForwardVector (Transformation|GetWorldRotation _capsule)) 7e+01)) (Utilities|Array|MakeArray "ObjectTypeQuery3") false 0 "None"))
        (if _returnvalue_2
          (Variables|CommonData|SetIn%20Attack%20Range (Actor|ActorHasTag (.HitActor (Collision|BreakHitResult _outhit)) "Player"))))
      (:then_1
        (if (not (Variables|CommonData|GetIn%20Attack%20Range))
          (Transformation|SetWorldLocation (Variables|Default|GetCapsule) (+ (Transformation|GetWorldLocation (Variables|Default|GetCapsule)) (Math|Vector|MakeVector 0.0 (* (Variables|CommonData|GetEnemy%20Speed) (Utilities|Time|GetWorldDeltaSeconds)) 0.0)) false false))))))

(event EventBeginPlay
  (if (Variables|CommonData|GetIs%20Enemy)
    (Transformation|SetWorldRotation (Variables|Default|GetCapsule self) "0.000000,-90.000000,0.000000" false false)
    (else
      (Transformation|SetWorldRotation (Variables|Default|GetCapsule self) "0.000000,90.000000,0.000000" false false))))

(event EventApplyDamage
  (params (Damage :type Integer))
  ;[1 1 1] Health
  (Development|PrintString (Utilities|String|ToString(Integer) Damage))
  (bind _output_get (Variables|Health|SetHealth (- (Variables|Health|GetHealth) Damage)))
  (if (<= _output_get 0.0)
    (Audio|PlaySoundatLocation 0 (Transformation|GetActorLocation) "0, 0, 0" 1.0 1.0 0.0 0 0 0 0)
    (Development|PrintString "Dead!")
    (Variables|Health|SetHealth 0.0)
    (if (Variables|CommonData|GetIs%20Enemy)
      (Default|CallControllerEnemyDestory (Variables|Default|GetControlller%20refer) self)
      (Actor|DestroyActor))
    (elif (> (Variables|Health|GetHealth) (Variables|Health|GetMax_Health))
      (Variables|Health|SetHealth (Variables|Health|GetMax_Health)))))

(fn ConstructionScript
  (bind _returnvalue (Utilities|GetDataTableRow "/Game/Piece/BluePrints/T_Chess.T_Chess" (Utilities|String|StringToName (Utilities|String|EnumtoString (Variables|CommonData|GetPawn%20Type))))
    (:then
      (Variables|Default|SetInitial%20Speed (.InitialSpeed (Utilities|Struct|BreakS_ChessData _returnvalue)))
      (Variables|Default|SetLife%20Span (.LifeSpan (Utilities|Struct|BreakS_ChessData _returnvalue)))
      (Variables|Default|SetDamage (.Damage (Utilities|Struct|BreakS_ChessData _returnvalue)))
      (Variables|Default|SetProject%20Gravity%20Scale (.ProjectGravityScale (Utilities|Struct|BreakS_ChessData _returnvalue)))
      (Variables|Default|SetFire%20Rate (.Firerate (Utilities|Struct|BreakS_ChessData _returnvalue)))
      (Components|Timeline|SetPlayRate (Variables|Default|GetTimeline) (Variables|Default|GetFire%20Rate))
      (Components|SkeletalMesh|SetSkeletalMeshAsset (Variables|Default|GetSkeletalMesh) (.Mesh (Utilities|Struct|BreakS_ChessData _returnvalue)))
      (Utilities|Array|Add (Variables|Actor|GetTags) (Utilities|String|StringToName (Utilities|String|EnumtoString (Variables|CommonData|GetFaction%20Tag))))
      (switch Utilities|FlowControl|Switch|SwitchonE_Faction (Variables|CommonData|GetFaction%20Tag)
        (:NewEnumerator0
          (Variables|CommonData|SetHit%20Target%20Actor "NewEnumerator1")
          (Variables|CommonData|SetIn%20Attack%20Range true))
        (:NewEnumerator1
          (Variables|CommonData|SetHit%20Target%20Actor "NewEnumerator0")
          (Variables|CommonData|SetIs%20Enemy true))))))

(fn RequestSlotData
  (return false "0, 0, 0"))