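; Enemy bullet projectile actor that damages what it overlaps and destroys itself on contact.
; A static mesh hit spawns a Niagara effect aligned to the surface normal and plays a sound, without applying damage.
; Capsule overlap applies damage to any overlapping actor without filtering, then plays damage effects and sounds.
; The construction script feeds speed, gravity scale and lifespan variables into the projectile movement and actor.
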(event OnComponentHit(StaticMesh)
  (params (HitComponent :type Primitive%20Component%20Object%20Reference) (OtherActor :type Actor%20Object%20Reference) (OtherComp :type Primitive%20Component%20Object%20Reference) (NormalImpulse :type Vector :default "0, 0, 0") (Hit :type Hit%20Result%20Structure%20%28by%20ref%29))
  (Variables|Default|SetHit Hit)
  (Niagara|SpawnSystematLocation 0 (.Location (Collision|BreakHitResult (Variables|Default|GetHit))) (Math|Rotator|MakeRotfromZ (.Normal (Collision|BreakHitResult (Variables|Default|GetHit)))) "0.200000,0.200000,0.200000")
  (Audio|PlaySoundatLocation 0 (.Location (Collision|BreakHitResult (Variables|Default|GetHit))) "0, 0, 0" 1.0 1.0 0.0 0 0 0 0)
  (Actor|DestroyActor))

(event OnComponentBeginOverlap(Capsule)
  (params (OverlappedComponent :type Primitive%20Component%20Object%20Reference) (OtherActor :type Actor%20Object%20Reference) (OtherComp :type Primitive%20Component%20Object%20Reference) (OtherBodyIndex :type Integer) (bFromSweep :type Boolean) (SweepResult :type Hit%20Result%20Structure%20%28by%20ref%29))
  (Game|Damage|ApplyDamage OtherActor (Variables|Default|GetBase%20Damage) 0 0)
  (CallFunction|PlayDMG))

(event Custom|PlayDMG
  (bind _staticmesh (Variables|Default|GetStaticMesh))
  (bind _returnvalue (Transformation|GetWorldLocation _staticmesh))
  (Audio|PlaySoundatLocation 0 _returnvalue "0, 0, 0" 1.0 1.0 0.0 0 0 0 0)
  (Niagara|SpawnSystematLocation 0 _returnvalue "0.000000,0.000000,-90.000000" "0.200000,0.200000,0.200000")
  (Niagara|SpawnSystematLocation 0 _returnvalue "0.000000,90.000000,0.000000")
  (Audio|PlaySoundatLocation 0 _returnvalue "0, 0, 0" 1.0 1.0 0.0 0 0 0 0)
  (Actor|DestroyActor))

(fn ConstructionScript
  (Variables|Default|SetBase%20Damage (Variables|Default|GetBase%20Damage))
  (Variables|/Script/Engine.ProjectileMovementComponent|SetInitialSpeed (Variables|Default|GetProjectileMovement) (Variables|Default|GetInitial%20Speed))
  (Variables|/Script/Engine.ProjectileMovementComponent|SetProjectileGravityScale (Variables|Default|GetProjectileMovement) (Variables|Default|GetProjectile%20Gravity%20Scale))
  (Actor|SetLifeSpan (Variables|Default|GetIn%20Lifespan)))