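; BP_Bullet is a projectile whose construction script sets initial speed, gravity scale and lifespan.
; On Sphere overlap, actors tagged with the HitTargetTag enum's name receive BaseDamage via ApplyDamageMessage and trigger PlayDMG effects and sounds, destroying the bullet if the Sphere is WorldDynamic.
; Other overlaps spawn normal-aligned impact effects and destroy it if the Sphere is WorldStatic; both type checks read the bullet's own component.
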(event OnComponentBeginOverlap(Sphere)
  (params (OverlappedComponent :type Primitive%20Component%20Object%20Reference) (OtherActor :type Actor%20Object%20Reference) (OtherComp :type Primitive%20Component%20Object%20Reference) (OtherBodyIndex :type Integer) (bFromSweep :type Boolean) (SweepResult :type Hit%20Result%20Structure%20%28by%20ref%29))
  (bind _output_get (Variables|Default|SetOverlapped%20Component OverlappedComponent))
  (if (Utilities|Array|ContainsItem (Variables|/Script/Engine.Actor|GetTags OtherActor) (Utilities|String|StringToName (Utilities|String|EnumtoString (Variables|Default|GetHit%20Target%20Tag))))
    (Class|BPIInteraction|ApplyDamage(Message) OtherActor (Variables|Default|GetBase%20Damage))
    (CallFunction|PlayDMG)
    (elif (Utilities|Enum|Equal(Enum) (Collision|GetCollisionObjectType _output_get) "ECC_WorldStatic")
      (Variables|Default|SetHit SweepResult)
      (Niagara|SpawnSystematLocation 0 (.Location (Collision|BreakHitResult (Variables|Default|GetHit))) (Math|Rotator|MakeRotfromZ (.Normal (Collision|BreakHitResult (Variables|Default|GetHit)))) "0.200000,0.200000,0.200000")
      (Audio|PlaySoundatLocation 0 (.Location (Collision|BreakHitResult (Variables|Default|GetHit))) "0, 0, 0" 1.0 1.0 0.0 0 0 0 0)
      (Actor|DestroyActor))))

(event Custom|PlayDMG
  (bind _staticmesh (Variables|Default|GetStaticMesh))
  (bind _returnvalue (Transformation|GetWorldLocation _staticmesh))
  (Audio|PlaySoundatLocation 0 _returnvalue "0, 0, 0" 1.0 1.0 0.0 0 0 0 0)
  (Niagara|SpawnSystematLocation 0 _returnvalue "0.000000,0.000000,-90.000000" "0.200000,0.200000,0.200000")
  (Niagara|SpawnSystematLocation 0 _returnvalue "0.000000,90.000000,0.000000")
  (Audio|PlaySoundatLocation 0 _returnvalue "0, 0, 0" 1.0 1.0 0.0 0 0 0 0)
  (if (Utilities|Enum|Equal(Enum) (Collision|GetCollisionObjectType (Variables|Default|GetOverlapped%20Component)) "ECC_WorldDynamic")
    (Actor|DestroyActor)))

(fn ConstructionScript
  (Variables|/Script/Engine.ProjectileMovementComponent|SetInitialSpeed (Variables|Default|GetProjectileMovement) (Variables|Default|GetInitial%20Speed))
  (Variables|/Script/Engine.ProjectileMovementComponent|SetProjectileGravityScale (Variables|Default|GetProjectileMovement) (Variables|Default|GetProjectile%20Gravity%20Scale))
  (Actor|SetLifeSpan (Variables|Default|GetIn%20Lifespan)))