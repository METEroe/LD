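; BP_KingArea is a box trigger area that registers a coin receive when the control piece enters it with its pickup flag set.
; Shortly after BeginPlay, it caches the player's ChessController and the BP_ControlPiece found in the level.
; On overlap by that piece, it calls CallControllerCoinReceive on the controller and clears PickUpFlag.
; The construction script sizes the box from the InBoxExtent variable.
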(event OnComponentBeginOverlap(Box)
  (params (OverlappedComponent :type Primitive%20Component%20Object%20Reference) (OtherActor :type Actor%20Object%20Reference) (OtherComp :type Primitive%20Component%20Object%20Reference) (OtherBodyIndex :type Integer) (bFromSweep :type Boolean) (SweepResult :type Hit%20Result%20Structure%20%28by%20ref%29))
  (if (== OtherActor (Variables|Default|GetAs%20BP%20Control%20Piece))
    (if (Variables|/Game/Piece/BluePrints/BP_ControlPiece.BP_ControlPiece_C|GetPickUpFlag (Variables|Default|GetAs%20BP%20Control%20Piece))
      (Default|CallControllerCoinReceive (Variables|Default|GetAs%20Chess%20Controller) 1)
      (Variables|/Game/Piece/BluePrints/BP_ControlPiece.BP_ControlPiece_C|SetPickUpFlag (Variables|Default|GetAs%20BP%20Control%20Piece) false))))

(event EventBeginPlay
  (Utilities|FlowControl|Delay 0.2)
  (bind _aschess_controller (Utilities|Casting|CastToChessController (Game|GetPlayerController 0)))
  (Variables|Default|SetAs%20Chess%20Controller _aschess_controller)
  (bind _returnvalue (Actor|GetActorOfClass 0))
  (bind _asbp_control_piece (Utilities|Casting|CastToBP_ControlPiece _returnvalue))
  (Variables|Default|SetAs%20BP%20Control%20Piece _asbp_control_piece))

(fn ConstructionScript
  (Variables|Default|SetIn%20Box%20Extent (Variables|Default|GetIn%20Box%20Extent))
  (Components|Box|SetBoxExtent (Variables|Default|GetBox) (Variables|Default|GetIn%20Box%20Extent) true))