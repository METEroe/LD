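; BP_Pickip is a pickup actor that a BP_ControlPiece collects by overlapping its capsule.
; BeginPlay announces the spawn with a pop sound and a Niagara burst, and Tick drives the mesh's relative Z with a sine intended as a bob.
; Overlap sets the piece's PickUpFlag, plays pickup feedback and destroys the actor, but only if that flag is not already set.
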(event OnComponentBeginOverlap(Capsule)
  (params (OverlappedComponent :type Primitive%20Component%20Object%20Reference) (OtherActor :type Actor%20Object%20Reference) (OtherComp :type Primitive%20Component%20Object%20Reference) (OtherBodyIndex :type Integer) (bFromSweep :type Boolean) (SweepResult :type Hit%20Result%20Structure%20%28by%20ref%29))
  (bind _asbp_control_piece (Utilities|Casting|CastToBP_ControlPiece OtherActor))
  (if (not (== (Variables|/Game/Piece/BluePrints/BP_ControlPiece.BP_ControlPiece_C|GetPickUpFlag _asbp_control_piece) true))
    (Variables|/Game/Piece/BluePrints/BP_ControlPiece.BP_ControlPiece_C|SetPickUpFlag _asbp_control_piece true)
    (Audio|PlaySound2D "/Game/SoundFX/Player/pickup2__greenvwbeetle__pop-5.pickup2__greenvwbeetle__pop-5" 1.0 1.0 0.0 0 0)
    (Niagara|SpawnSystematLocation "/Game/VFX/NS_DotUp.NS_DotUp" (Transformation|GetWorldLocation (Variables|Default|GetCapsule)))
    (Actor|DestroyActor)))

(event EventBeginPlay
  (Audio|PlaySound2D "/Game/SoundFX/Death/death1__zmb94__pop1.death1__zmb94__pop1" 1.0 1.0 0.0 0 0)
  (Niagara|SpawnSystematLocation "/Game/ToolKit/NiagaraSystems/ColorChange+RefractionExplode/NS_ColoredHexagon+RefractParasyteExplosion.NS_ColoredHexagon+RefractParasyteExplosion" (Transformation|GetWorldLocation (Variables|Default|GetCapsule))))

(event EventTick
  (params (DeltaSeconds :type Float%20%28single-precision%29))
  (bind _output_get (Variables|Default|SetDelta%20Seconds (+ DeltaSeconds (Variables|Default|GetDelta%20Seconds))))
  (Transformation|SetRelativeLocation (Variables|Default|GetStaticMesh) (Math|Vector|MakeVector 0.0 0.0 (* (Math|Trig|Sin(Radians) _output_get) 3e+01)) false false))

(fn ConstructionScript)