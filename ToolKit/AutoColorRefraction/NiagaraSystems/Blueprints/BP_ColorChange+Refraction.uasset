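; Configurable Niagara effect actor with sparks, refraction and an optional MetaSound, active from BeginPlay or toggled by box overlap.
; Construction script and each activation push exposed spark, refraction, noise, fade and mesh settings into Niagara user variables, optionally showing the source static mesh.
; With AutoActivate off, any actor entering the box starts the effect and leaving stops effect and sound.
; SoundActivated gates the audio.
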(event OnComponentBeginOverlap(Box)
  (params (OverlappedComponent :type Primitive%20Component%20Object%20Reference) (OtherActor :type Actor%20Object%20Reference) (OtherComp :type Primitive%20Component%20Object%20Reference) (OtherBodyIndex :type Integer) (bFromSweep :type Boolean) (SweepResult :type Hit%20Result%20Structure%20%28by%20ref%29))
  (CallFunction|GetSoundActivated?)
  (if (not (Variables|GeneralParameters:|GetAutoActivate?))
    (Components|Activation|SetActive (Variables|Default|GetNiagara) true false)
    (CallFunction|NiagaraColorChange+RefractionParameters)
    (CallFunction|GetSoundActivated?)))

(event OnComponentEndOverlap(Box)
  (params (OverlappedComponent :type Primitive%20Component%20Object%20Reference) (OtherActor :type Actor%20Object%20Reference) (OtherComp :type Primitive%20Component%20Object%20Reference) (OtherBodyIndex :type Integer))
  (CallFunction|GetSoundActivated?)
  (if (not (Variables|GeneralParameters:|GetAutoActivate?))
    (Components|Activation|SetActive (Variables|Default|GetNiagara) false false)))

(event EventBeginPlay
  (bind _niagara (Variables|Default|GetNiagara))
  (Audio|Components|Audio|SetSound (Variables|Default|GetMetasound) (Variables|GeneralParameters:|GetSound))
  (CallFunction|GetSoundActivated?)
  (if (Variables|GeneralParameters:|GetAutoActivate?)
    (Components|Activation|SetActive _niagara true false)
    (CallFunction|NiagaraColorChange+RefractionParameters)
    (CallFunction|GetSoundActivated?)
    (else
      (Components|Activation|SetActive _niagara false false))))

(fn ConstructionScript
  (CallFunction|NiagaraColorChange+RefractionParameters))

(fn NiagaraColorChange+RefractionParameters
  (bind _niagara (Variables|Default|GetNiagara))
  (bind _staticmeshparticle (Variables|GeneralParameters:|GetStaticMeshParticle))
  (bind _staticmesh (Variables|Default|GetStaticMesh))
  (Class|NiagaraComponent|SetAsset (Variables|Default|GetNiagara) (Variables|GeneralParameters:|GetNiagaraSystem) true)
  (if (Variables|GeneralParameters:|GetStaticMeshVisible)
    (Components|StaticMesh|SetStaticMesh _staticmesh _staticmeshparticle)
    (Rendering|SetVisibility _staticmesh true false)
    (else
      (Components|StaticMesh|SetStaticMesh _staticmesh _staticmeshparticle)
      (Rendering|SetVisibility _staticmesh false false)))
  (Class|NiagaraFunctionLibrary|OverrideSystemUserVariableStaticMesh _niagara "StaticMeshParticle" _staticmeshparticle)
  (Niagara|SetNiagaraVariable(Vector3) _niagara "SparkOffset" (Variables|ParticlesParameters:|GetSparkOffset))
  (Niagara|SetNiagaraVariable(Float) _niagara "Camera Offset" (Variables|ParticlesParameters:|GetCamera%20Offset))
  (Niagara|SetNiagaraVariable(Float) _niagara "DrawMaxDistance" (Variables|GeneralParameters:|GetFadeDistance))
  (Niagara|SetNiagaraVariable(Float) _niagara "Noise Strength" (Variables|ParticlesParameters:|GetNoise%20Strength))
  (Niagara|SetNiagaraVariable(Float) _niagara "Spark1Quantity" (Variables|ParticlesParameters:|GetSpark1Quantity))
  (Niagara|SetNiagaraVariable(Float) _niagara "Spark1ScaleMax" (Variables|ParticlesParameters:|GetSpark1ScaleMax))
  (Niagara|SetNiagaraVariable(Float) _niagara "Spark1ScaleMin" (Variables|ParticlesParameters:|GetSpark1ScaleMin))
  (Niagara|SetNiagaraVariable(Float) _niagara "Spark2Quantity" (Variables|ParticlesParameters:|GetSpark2Quantity))
  (Niagara|SetNiagaraVariable(Float) _niagara "Spark2ScaleMax" (Variables|ParticlesParameters:|GetSpark2ScaleMax))
  (Niagara|SetNiagaraVariable(Float) _niagara "Spark2ScaleMin" (Variables|ParticlesParameters:|GetSpark2ScaleMin))
  (Niagara|SetNiagaraVariable(Float) _niagara "SparkOffsetScale" (Variables|ParticlesParameters:|GetSparkOffsetScale))
  (Niagara|SetNiagaraVariable(Float) _niagara "VelocitySpeedMax" (Variables|ParticlesParameters:|GetVelocitySpeedMax))
  (Niagara|SetNiagaraVariable(Float) _niagara "VelocitySpeedMin" (Variables|ParticlesParameters:|GetVelocitySpeedMin))
  (Niagara|SetNiagaraVariable(Float) _niagara "RefractionAmount" (Variables|RefractionPrarmeters:|GetRefractionAmount))
  (Niagara|SetNiagaraVariable(Float) _niagara "RefractionScaleMax" (Variables|RefractionPrarmeters:|GetRefractionScaleMax))
  (Niagara|SetNiagaraVariable(Float) _niagara "RefractionScaleMin" (Variables|RefractionPrarmeters:|GetRefractionScaleMin))
  (Niagara|SetNiagaraVariable(Float) _niagara "RefractionVelocityMax" (Variables|RefractionPrarmeters:|GetRefractionVelocityMax))
  (Niagara|SetNiagaraVariable(Float) _niagara "RefractionVelocityMin" (Variables|RefractionPrarmeters:|GetRefractionVelocityMin))
  (Niagara|SetNiagaraVariable(Float) _niagara "Refraction Noise Strength" (Variables|RefractionPrarmeters:|GetRefraction%20Noise%20Strength)))

(fn GetSoundActivated?
  (bind _metasound (Variables|Default|GetMetasound))
  (if (Variables|GeneralParameters:|GetSoundActivated)
    (Components|Activation|SetActive _metasound true false)
    (else
      (Components|Activation|SetActive _metasound false false))))