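; Showcase actor for a Niagara colour-change and refraction explosion effect that can burst from a static mesh, with optional sound.
; The construction script, BeginPlay and a Level Sequence event all push exposed mesh, spark and refraction settings into Niagara user parameters.
; With box overlap enabled, entering activates the effect and optional Metasound once, then hides the mesh and disables its collision after a delay.
; Leaving re-arms the trigger and deactivates both.
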(event OnComponentBeginOverlap(Box)
  (params (OverlappedComponent :type Primitive%20Component%20Object%20Reference) (OtherActor :type Actor%20Object%20Reference) (OtherComp :type Primitive%20Component%20Object%20Reference) (OtherBodyIndex :type Integer) (bFromSweep :type Boolean) (SweepResult :type Hit%20Result%20Structure%20%28by%20ref%29))
  (bind _staticmesh (Variables|Default|GetStaticMesh))
  (bind _delaybeforestaticmeshdisappears (Variables|GeneralParameters:|GetDelayBeforeStaticMeshDisappears))
  (if (Variables|GeneralParameters:|GetUseBoxOverlap)
    (Utilities|FlowControl|DoOnce false
      (:Completed
        (Components|Activation|SetActive (Variables|Default|GetNiagara) true false)
        (if (Variables|GeneralParameters:|GetSoundActivated)
          (Components|Activation|SetActive (Variables|Default|GetMetasound) true false))
        (Utilities|FlowControl|Delay _delaybeforestaticmeshdisappears)
        (if (!= _delaybeforestaticmeshdisappears -1.0)
          (Rendering|SetVisibility _staticmesh false false)
          (Collision|SetCollisionEnabled _staticmesh "NoCollision"))))))

(event OnComponentEndOverlap(Box)
  (params (OverlappedComponent :type Primitive%20Component%20Object%20Reference) (OtherActor :type Actor%20Object%20Reference) (OtherComp :type Primitive%20Component%20Object%20Reference) (OtherBodyIndex :type Integer))
  (bind _metasound (Variables|Default|GetMetasound))
  (bind _niagara (Variables|Default|GetNiagara))
  (bind _staticmesh (Variables|Default|GetStaticMesh))
  (bind _delaybeforestaticmeshdisappears (Variables|GeneralParameters:|GetDelayBeforeStaticMeshDisappears))
  (Utilities|FlowControl|Sequence
    (:then_0
      (Utilities|FlowControl|DoOnce false) ; enters at Reset
    )
    (:then_1
      (Components|Activation|SetActive _niagara false false)
      (Components|Activation|SetActive _metasound false false))))

(event Custom|ModifyParameters
  ;[1 1 1] Used to call modification during Showcase Level Sequence, can be deleted for your own project
  (CallFunction|NiagaraColorChange+RefractionExplodeParameters))

(event EventBeginPlay
  (Audio|Components|Audio|SetSound (Variables|Default|GetMetasound) (Variables|GeneralParameters:|GetSound))
  (CallFunction|NiagaraColorChange+RefractionExplodeParameters))

(fn ConstructionScript
  (CallFunction|NiagaraColorChange+RefractionExplodeParameters))

(fn NiagaraColorChange+RefractionExplodeParameters
  (bind _niagara (Variables|Default|GetNiagara))
  (bind _staticmeshparticle (Variables|GeneralParameters:|GetStaticMeshParticle))
  (bind _staticmesh (Variables|Default|GetStaticMesh))
  (Class|NiagaraComponent|SetAsset (Variables|Default|GetNiagara) (Variables|GeneralParameters:|GetNiagaraSystem) true)
  (if (Variables|GeneralParameters:|GetStaticMeshVisible)
    (Components|StaticMesh|SetStaticMesh _staticmesh _staticmeshparticle)
    (Rendering|SetVisibility _staticmesh true false)
    (else
      (Components|StaticMesh|SetStaticMesh _staticmesh _staticmeshparticle)
      (Rendering|SetVisibility _staticmesh false false)))
  (Class|NiagaraFunctionLibrary|OverrideSystemUserVariableStaticMesh _niagara "StaticMeshParticle" _staticmeshparticle)
  (Niagara|SetNiagaraVariable(Vector3) _niagara "SparkOffset" (Variables|ParticlesParameters:|GetSparkOffset))
  (Niagara|SetNiagaraVariable(Float) _niagara "Camera Offset" (Variables|ParticlesParameters:|GetCamera%20Offset))
  (Niagara|SetNiagaraVariable(Float) _niagara "DrawMaxDistance" (Variables|GeneralParameters:|GetFadeDistance))
  (Niagara|SetNiagaraVariable(Float) _niagara "Noise Strength" (Variables|ParticlesParameters:|GetNoise%20Strength))
  (Niagara|SetNiagaraVariable(Float) _niagara "Spark1Quantity" (Variables|ParticlesParameters:|GetSpark1Quantity))
  (Niagara|SetNiagaraVariable(Float) _niagara "Spark1ScaleMax" (Variables|ParticlesParameters:|GetSpark1ScaleMax))
  (Niagara|SetNiagaraVariable(Float) _niagara "Spark1ScaleMin" (Variables|ParticlesParameters:|GetSpark1ScaleMin))
  (Niagara|SetNiagaraVariable(Float) _niagara "Spark2Quantity" (Variables|ParticlesParameters:|GetSpark2Quantity))
  (Niagara|SetNiagaraVariable(Float) _niagara "Spark2ScaleMax" (Variables|ParticlesParameters:|GetSpark2ScaleMax))
  (Niagara|SetNiagaraVariable(Float) _niagara "Spark2ScaleMin" (Variables|ParticlesParameters:|GetSpark2ScaleMin))
  (Niagara|SetNiagaraVariable(Float) _niagara "SparkOffsetScale" (Variables|ParticlesParameters:|GetSparkOffsetScale))
  (Niagara|SetNiagaraVariable(Float) _niagara "VelocitySpeedMax" (Variables|ParticlesParameters:|GetVelocitySpeedMax))
  (Niagara|SetNiagaraVariable(Float) _niagara "VelocitySpeedMin" (Variables|ParticlesParameters:|GetVelocitySpeedMin))
  (Niagara|SetNiagaraVariable(Float) _niagara "RefractionAmount" (Variables|RefractionPrarmeters:|GetRefractionAmount))
  (Niagara|SetNiagaraVariable(Float) _niagara "RefractionScaleMax" (Variables|RefractionPrarmeters:|GetRefractionScaleMax))
  (Niagara|SetNiagaraVariable(Float) _niagara "RefractionScaleMin" (Variables|RefractionPrarmeters:|GetRefractionScaleMin))
  (Niagara|SetNiagaraVariable(Float) _niagara "RefractionVelocityMax" (Variables|RefractionPrarmeters:|GetRefractionVelocityMax))
  (Niagara|SetNiagaraVariable(Float) _niagara "RefractionVelocityMin" (Variables|RefractionPrarmeters:|GetRefractionVelocityMin))
  (Niagara|SetNiagaraVariable(Float) _niagara "Refraction Noise Strength" (Variables|RefractionPrarmeters:|GetRefraction%20Noise%20Strength))
  (Niagara|SetNiagaraVariable(Float) _niagara "Refraction Loop Duration" (Variables|RefractionPrarmeters:|GetRefraction%20Loop%20Duration))
  (Niagara|SetNiagaraVariable(Vector3) _niagara "Spark1GravityMax" (Variables|ParticlesParameters:|GetSpark1GravityMax))
  (Niagara|SetNiagaraVariable(Vector3) _niagara "Spark1GravityMin" (Variables|ParticlesParameters:|GetSpark1GravityMin))
  (Niagara|SetNiagaraVariable(Float) _niagara "Spark1Loop Duration" (Variables|ParticlesParameters:|GetSpark1Loop%20Duration))
  (Niagara|SetNiagaraVariable(Vector3) _niagara "Spark2GravityMax" (Variables|ParticlesParameters:|GetSpark2GravityMax))
  (Niagara|SetNiagaraVariable(Vector3) _niagara "Spark2GravityMin" (Variables|ParticlesParameters:|GetSpark2GravityMin))
  (Niagara|SetNiagaraVariable(Float) _niagara "Spark2Loop Duration" (Variables|ParticlesParameters:|GetSpark2Loop%20Duration)))