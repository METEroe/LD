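; Editor-side generated dynamic mesh actor that builds a damaged version of a static mesh with Geometry Script.
; A copy of the mesh becomes a boolean tool, smoothed by morphology passes, roughened by seeded Perlin noise layers and box-projected for an internal material.
; It intersects with the remeshed, optionally shelled original, leaving damaged areas with that material.
; ConverttoStaticMesh bakes the result to a new asset, optionally Nanite, and replaces the actor.
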(event Custom|Execute%20Boolean
  ;[1 1 1] boolean
  (GeometryScript|Booleans|ApplyMeshBoolean :TargetMesh (Variables|System|GetDynamic%20Mesh) :ToolMesh (Variables|System|GetBoolean%20Dynamic%20Mesh) :Operation "Intersection" :Options (Utilities|Struct|MakeGeometryScriptMeshBooleanOptions true true 0.01) :Debug 0))

(event Custom|Make%20Boolean%20Mesh
  ;[0 0 0] boolean tool
  (bind _returnvalue (DynamicMeshActor|AllocateComputeMesh))
  (Variables|System|SetBoolean%20Dynamic%20Mesh _returnvalue)
  (GeometryScript|StaticMesh|CopyMeshFromStaticMesh :FromStaticMeshAsset (Variables|Settings|GetStatic%20Mesh) :ToDynamicMesh (Variables|System|GetBoolean%20Dynamic%20Mesh) :Debug 0
    (:Success
      (Class|GeometryScriptLibraryMeshRepairFunctions|WeldMeshEdges (Variables|System|GetBoolean%20Dynamic%20Mesh) (Utilities|Struct|MakeGeometryScriptWeldEdgesOptions 0.001 false) 0)
      ;;[0.9416 1 0] material id
      (bind _materialindex (Class|GeometryScriptLibraryStaticMeshFunctions|GetSectionMaterialListfromStaticMesh :FromStaticMeshAsset (Variables|Settings|GetStatic%20Mesh) :Debug 0)
        (:Success
          (bind _output_get (Variables|System|SetInternals%20Material%20ID (+ (Utilities|Array|LastIndex _materialindex) 1)))
          (GeometryScript|Materials|RemapMaterialIDs (Variables|System|GetBoolean%20Dynamic%20Mesh) 0 _output_get 0)
          ;;[0 1 0.803] smooth
          (for _index (range 0 2)
            (Class|GeneratedDynamicMeshActor|IncrementProgress 1 "Building Mesh...")
            (bind _returnvalue_2 (Class|GeometryScriptLibraryMeshVoxelFunctions|ApplyMeshMorphology (Variables|System|GetBoolean%20Dynamic%20Mesh) (Utilities|Struct|MakeGeometryScriptMorphologyOptions (Utilities|Struct|MakeGeometryScript3DGridParameters "GridResolution" 0.5 (+ (* _index 20) (Class|KismetSystemLibrary|MakeLiteralInteger (Variables|Settings|GetInternal%20Resolution)))) false "(SizeMethod=GridResolution,GridCellSize=0.500000,GridResolution=64)" "Dilate" (Variables|Settings|GetDistance)) 0))
            (Class|GeometryScriptLibraryMeshDeformFunctions|ApplyIterativeSmoothingtoMesh :TargetMesh _returnvalue_2 :Options (Utilities|Struct|MakeGeometryScriptIterativeMeshSmoothingOptions (Variables|Settings|GetChamfer%20Scale) 0.2 "FullMeshSelection") :Debug 0))
          ;;[1 0.906 0.3704] UVs
          (Class|GeometryScriptLibraryMeshUVFunctions|SetMeshUVsfromBoxProjection :TargetMesh (Variables|System|GetBoolean%20Dynamic%20Mesh) :BoxTransform (Math|Transform|MakeTransform "0, 0, 0" "0.000000,0.000000,45.000000" (Variables|Settings|GetInternal%20UV%20Scale)) :Debug 0)
          (GeometryScript|Materials|RemapMaterialIDs (Variables|System|GetBoolean%20Dynamic%20Mesh) 0 (Variables|System|GetInternals%20Material%20ID) 0))))))

(event Custom|Convert%20to%20Static%20Mesh
  (params (Nanite :type Boolean))
  (bind _returnvalue (GeometryScript|AssetManagement|CreateNewStaticMeshAssetfromMesh (Variables|System|GetDynamic%20Mesh) (Utilities|String|Append (.LeftS (Utilities|String|Split (Class|KismetSystemLibrary|GetPathName (Variables|Settings|GetStatic%20Mesh)) ".")) (Utilities|String|Append "_Destroyed-" (Utilities|String|ToString(Integer) (Class|KismetMathLibrary|RandomIntegerfromStream (Variables|Settings|GetSeed) 9999)))) (Utilities|Struct|MakeGeometryScriptCreateNewStaticMeshAssetOptions false false Nanite (Utilities|Struct|MakeMeshNaniteSettings Nanite) 0.0 true) 0)
    (:Success
      (for (_array_element _array_index) (Rendering|Material|GetMaterials (Variables|DynamicMeshActor|GetDynamicMeshComponent))
        (Rendering|Material|SetMaterial _returnvalue _array_index _array_element))
      (bind _returnvalue_2 (Game|SpawnActorfromClass "/Script/Engine.StaticMeshActor" (Transformation|GetActorTransform) "Undefined" "MultiplyWithRoot" 0 0))
      (Components|StaticMesh|SetStaticMesh (Variables|/Script/Engine.StaticMeshActor|GetStaticMeshComponent _returnvalue_2) _returnvalue)
      (Actor|DestroyActor))))

(event Events|EventOnRebuildGeneratedMesh
  (params (TargetMesh :type Dynamic%20Mesh%20Object%20Reference))
  (Variables|System|SetDynamic%20Mesh TargetMesh)
  ;[1 1 1] progress increment count
  (Variables|Default|SetNumProgressSteps (+ (Class|KismetSystemLibrary|MakeLiteralInteger 8) (Utilities|Array|Length (Variables|Settings|GetNoise))))
  (Class|GeneratedDynamicMeshActor|IncrementProgress 1 "Building Mesh...")
  ;[0.1264 0.4293 1] Copy static mesh
  (GeometryScript|StaticMesh|CopyMeshFromStaticMesh :FromStaticMeshAsset (Variables|Settings|GetStatic%20Mesh) :ToDynamicMesh (Variables|System|GetDynamic%20Mesh) :AssetOptions (Utilities|Struct|MakeGeometryScriptCopyMeshfromAssetOptions false false) :Debug 0
    (:Success
      ;[1 1 1] shell based on thickness value
      (if (== (Variables|Settings|GetThickness) 0.0)
        _
        (else
          (Class|GeometryScriptLibraryMeshModelingFunctions|ApplyMeshShell (Variables|System|GetDynamic%20Mesh) (Utilities|Struct|MakeGeometryScriptMeshOffsetOptions (* (Variables|Settings|GetThickness) -1.0) false 5 0.0 false 0.001) 0)))
      (Class|GeometryScriptLibraryRemeshingFunctions|ApplyUniformRemesh :TargetMesh (Variables|System|GetDynamic%20Mesh) :Debug 0)
      (Utilities|FlowControl|Sequence
        (:then_0
          (Class|GeneratedDynamicMeshActor|IncrementProgress 1 "Building Mesh..."))
        (:then_1
          (CallFunction|MakeBooleanMesh))
        (:then_2
          (if (Variables|Settings|GetForce%20Bevel)
            (CallFunction|ExecuteBoolean)))
        (:then_3
          (Class|GeometryScriptLibraryMeshModelingFunctions|ApplyMeshOffset (Variables|System|GetDynamic%20Mesh) (Utilities|Struct|MakeGeometryScriptMeshOffsetOptions (Variables|Settings|GetInflate) false 5 0.1 false 0.2) 0))
        (:then_4
          ;[1 0.05208 0.5266] noise
          (for _array_element (Variables|Settings|GetNoise)
            (Class|GeneratedDynamicMeshActor|IncrementProgress 1 "Building Mesh...")
            (Class|GeometryScriptLibraryMeshDeformFunctions|ApplyPerlinNoisetoMesh :TargetMesh (Variables|System|GetBoolean%20Dynamic%20Mesh) :Options (Utilities|Struct|MakeGeometryScriptPerlinNoiseOptions (Utilities|Struct|MakeGeometryScriptPerlinNoiseLayerOptions (.Magnitude (Utilities|Struct|BreakST_NoiseSettings _array_element)) (.Frequency (Utilities|Struct|BreakST_NoiseSettings _array_element)) (.Offset (Utilities|Struct|BreakST_NoiseSettings _array_element)) (Class|KismetMathLibrary|RandomIntegerfromStream (Variables|Settings|GetSeed) 999)) true "FullMeshSelection") :Debug 0))
          (Class|GeometryScriptLibraryRemeshingFunctions|ApplyUniformRemesh (Variables|System|GetBoolean%20Dynamic%20Mesh) (Utilities|Struct|MakeGeometryScriptRemeshOptions true true) (Utilities|Struct|MakeGeometryScriptUniformRemeshOptions "TriangleCount" 50000 1.0) 0)
          (GeometryScript|Materials|RemapMaterialIDs (Variables|System|GetBoolean%20Dynamic%20Mesh) 0 (Variables|System|GetInternals%20Material%20ID) 0)
          ;[1 0.906 0.3704] UVs
          (Class|GeometryScriptLibraryMeshUVFunctions|SetMeshUVsfromBoxProjection :TargetMesh (Variables|System|GetBoolean%20Dynamic%20Mesh) :BoxTransform (Math|Transform|MakeTransform "0, 0, 0" "0, 0, 0" (Variables|Settings|GetInternal%20UV%20Scale)) :Debug 0))
        (:then_5
          (Class|GeneratedDynamicMeshActor|IncrementProgress 1 "Building Mesh..."))
        (:then_6
          (CallFunction|ExecuteBoolean))
        (:then_7
          (Class|GeneratedDynamicMeshActor|IncrementProgress 1 "Setting Materials..."))
        (:then_8
          ;[0.03839 0.1943 1] set materials
          (bind _materiallist (Class|GeometryScriptLibraryStaticMeshFunctions|GetSectionMaterialListfromStaticMesh :FromStaticMeshAsset (Variables|Settings|GetStatic%20Mesh) :Debug 0)
            (:Success
              (Variables|System|SetMaterial%20List _materiallist)
              (Utilities|Array|Add (Variables|System|GetMaterial%20List) "/Game/ToolKit/MeshDamageToolkit/Material/Internal/MI_Internal.MI_Internal")
              (Class|DynamicMeshComponent|ConfigureMaterialSet (Variables|DynamicMeshActor|GetDynamicMeshComponent) (Variables|System|GetMaterial%20List)))))
        (:then_9
          (Class|GeneratedDynamicMeshActor|IncrementProgress 1 "Cleaning..."))
        (:then_10
          ;[1 1 1] cleaning
          (DynamicMeshActor|ReleaseAllComputeMeshes))))))

(fn ConstructionScript
  (Variables|Default|SetbFrozen (Variables|Settings|GetFrozen)))