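; Player character for a prototype with grab-and-assemble interaction, showing a control-tips widget and mouse cursor.
; Input handlers forward clicking, grab rotation and height, assembly mode, constraint breaking and saving to BPInteraction.
; While BPInteraction has an InteractionActor, forward input drives that actor, and strafing and jumping are blocked.
; Actors in interact range register in InTriggerRangeActor, and F triggers a random one, despite a comment intending nearest or highest-weighted.
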(event EventTick
  (params (DeltaSeconds :type Float%20%28single-precision%29))
  ;[0.724 0.1506 0.165] 摄象机旋转与移动功能暂时不做，因为游戏原型没有确定
)

(event EventBeginPlay
  (bind _returnvalue (Game|GetPlayerController 0))
  (bind _returnvalue_2 (UserInterface|CreateWidget "/Game/BP/Widget/WBP_ControlTips.WBP_ControlTips_C"))
  (UserInterface|Viewport|AddtoViewport _returnvalue_2 0)
  (Input|SetInputModeGameandUI _returnvalue 0 "DoNotLock" true false)
  (Variables|/Script/Engine.PlayerController|SetbShowMouseCursor _returnvalue true))

(event EventAddtoInteractRange
  (params (To%20add%20actor :type Actor%20Object%20Reference))
  ;[0.6832 0.7239 0.8542] 在交互对象进入/离开范围内时触发，可以建立Map来管理需要呈现的Widget
  (Utilities|Array|Add (Variables|Default|GetIn%20Trigger%20Range%20Actor) To%20add%20actor))

(event EventRemovefromInteractRange
  (params (To%20remove%20actor :type Actor%20Object%20Reference))
  ;[0.6832 0.7239 0.8542] 在交互对象进入/离开范围内时触发，可以建立Map来管理需要呈现的Widget
  (Utilities|Array|RemoveItem (Variables|Default|GetIn%20Trigger%20Range%20Actor) To%20remove%20actor))

(event Input|ActionEvents|InputActionJump
  (params (Key :type Key%20Structure :default "None"))
  ;[0 0.4737 1] Movement input   玩家移动输入，当玩家操纵控制杆时不移动，输入传给控制杆
  (:Pressed
    (Utilities|IsValid (Variables|/Game/BP/BPC_Interaction.BPC_Interaction_C|GetInteractionActor (Variables|Default|GetBP_Interaction))
      (:Is%20Not%20Valid
        (Character|Jump))))
  (:Released
    (Character|StopJumping)))

(event Input|AxisEvents|InputAxisGrapRotateUp
  (params (AxisValue :type Float%20%28single-precision%29))
  ;[0.6707 0.7106 0.8385] 操作抓取物
  (Default|ModifyGrapRotateUp (Variables|Default|GetBP_Interaction) AxisValue))

(event Input|AxisEvents|InputAxisGrapRotateRight
  (params (AxisValue :type Float%20%28single-precision%29))
  ;[0.6707 0.7106 0.8385] 操作抓取物
  (Default|ModifyGrapRotateRight (Variables|Default|GetBP_Interaction) AxisValue))

(event Input|AxisEvents|InputAxisGrapDistance
  (params (AxisValue :type Float%20%28single-precision%29))
  ;[0.6707 0.7106 0.8385] 操作抓取物
  (Default|ModifyGrapHeight (Variables|Default|GetBP_Interaction) AxisValue))

(event Input|AxisEvents|InputAxisMoveForward
  (params (AxisValue :type Float%20%28single-precision%29))
  (bind _bp_interaction (Variables|Default|GetBP_Interaction))
  (bind _interactionactor (Variables|/Game/BP/BPC_Interaction.BPC_Interaction_C|GetInteractionActor _bp_interaction))
  ;[0 0.4737 1] Movement input   玩家移动输入，当玩家操纵控制杆时不移动，输入传给控制杆
  (Utilities|IsValid _interactionactor
    (:Is%20Valid
      (Class|BPIPhysicInteraction|DriveTarget(Message) _interactionactor (Math|Vector2D|MakeVector2D AxisValue (stale Input|AxisEvents|InputAxisMoveRight AxisValue))))
    (:Is%20Not%20Valid
      (Pawn|Input|AddMovementInput "1.000000,0.000000,0.000000" AxisValue false))))

(event Input|AxisEvents|InputAxisMoveRight
  (params (AxisValue :type Float%20%28single-precision%29))
  ;[0 0.4737 1] Movement input   玩家移动输入，当玩家操纵控制杆时不移动，输入传给控制杆
  (Utilities|IsValid (Variables|/Game/BP/BPC_Interaction.BPC_Interaction_C|GetInteractionActor (Variables|Default|GetBP_Interaction))
    (:Is%20Not%20Valid
      (Pawn|Input|AddMovementInput "0.000000,1.000000,0.000000" AxisValue false))))

(event Input|KeyboardEvents|F
  (params (Key :type Key%20Structure :default "None"))
  ;[0.6832 0.7239 0.8542] 在进入Trigger后，按下F触发对象的逻辑。选择其中最近的一个或者权重最高的一个
  (:Pressed
    (Class|BPIInteraction|InteracttoTarget(Message) (.OutItem (Utilities|Array|Random (Variables|Default|GetIn%20Trigger%20Range%20Actor))) "NewEnumerator1")))

(event Input|KeyboardEvents|X
  (params (Key :type Key%20Structure :default "None"))
  ;[0.6707 0.7106 0.8385] 操作抓取物
  (:Pressed
    (Default|BreakConstraint (Variables|Default|GetBP_Interaction))))

(event Input|KeyboardEvents|Z
  (params (Key :type Key%20Structure :default "None"))
  ;[0.6707 0.7106 0.8385] 操作抓取物
  (:Pressed
    (Default|SwitchAssmblyMode (Variables|Default|GetBP_Interaction))))

(event Input|KeyboardEvents|CtrlS
  (params (Key :type Key%20Structure :default "None"))
  ;[0.6707 0.7106 0.8385] 操作抓取物
  (:Pressed
    (Default|SaveCurrentGrapModuler (Variables|Default|GetBP_Interaction))))

(event Input|KeyboardEvents|C
  (params (Key :type Key%20Structure :default "None"))
  ;[0.6707 0.7106 0.8385] 操作抓取物
  (:Pressed
    (Default|CheckSaveData (Variables|Default|GetBP_Interaction))))

(event Input|MouseEvents|LeftMouseButton
  (params (Key :type Key%20Structure :default "None"))
  ;[0.6707 0.7106 0.8385] 操作抓取物
  (:Pressed
    (Default|ClickActor (Variables|Default|GetBP_Interaction))))

(fn ConstructionScript)

(fn RequestCharacterRefer
  (return 0))