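; BP_MaterialManager temporarily overrides the materials on a set of components and restores their originals.
; SaveInitMaterial caches each component's materials by slot index in the MaterialInfo map, using a struct-wrapped inner map.
; SetMaterial either restores and clears that cache, or fills every slot with a dynamic instance of NewMaterial created through Owner.
; Its vector parameter call uses the name None and runs before each new material is assigned.
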(event Custom|SetMaterial
  (params (ResetToInit :type Boolean) (Component :type Array%20of%20Primitive%20Component%20Object%20References) (NewMaterial :type Material%20Interface%20Object%20Reference) (Parameter :type Vector))
  (bind _materialinfo (Variables|Default|GetMaterialInfo))
  (if ResetToInit
    (Utilities|FlowControl|Sequence
      (:then_0
        (bind _keys (Utilities|Map|Keys _materialinfo))
        (for _array_element _keys
          (bind _keys_2 (Utilities|Map|Keys (Utilities|Struct|BreakS_MapMaterial (.Value (Utilities|Map|Find _materialinfo _array_element)))))
          (for _array_element_2 _keys_2
            (Rendering|Material|SetMaterial _array_element _array_element_2 (.Value (Utilities|Map|Find (Utilities|Struct|BreakS_MapMaterial (.Value (Utilities|Map|Find _materialinfo _array_element))) _array_element_2))))))
      (:then_1
        (Utilities|Map|Clear (Variables|Default|GetMaterialInfo))))
    (else
      (for _array_element_3 Component
        (for _index (range 0 (- (Rendering|Material|GetNumMaterials _array_element_3) 1))
          (bind _returnvalue (Default|CreateDyncMaterial (Variables|Default|GetOwner) NewMaterial "None" "None"))
          (Rendering|Material|SetVectorParameterValueonMaterials (.AsMesh%20Component (Utilities|Casting|CastToMeshComponent _array_element_3)) "None" Parameter)
          (Rendering|Material|SetMaterial _array_element_3 _index _returnvalue))))))

(event Custom|SaveInitMaterial
  (params (Component :type Array%20of%20Primitive%20Component%20Object%20References))
  (for _array_element Component
    (for _index (range 0 (- (Rendering|Material|GetNumMaterials _array_element) 1))
      (Utilities|Map|Add (Utilities|Struct|BreakS_MapMaterial (Variables|Default|GetcacheMaterial)) _index (Rendering|Material|GetMaterial _array_element _index)))
    (Utilities|Map|Add (Variables|Default|GetMaterialInfo) _array_element (Variables|Default|GetcacheMaterial))
    (Utilities|Map|Clear (Utilities|Struct|BreakS_MapMaterial (Variables|Default|GetcacheMaterial)))))