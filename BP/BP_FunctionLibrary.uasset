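; Blueprint function library for a physics assembly system where mesh parts are glued into groups and snapped together.
; A mesh's first component tag keys its group record in the player's BPC_Interaction, driving group lookup, registration and physics toggling with interface overrides.
; Rotation snapping picks the closest orientation from transformed axis and diagonal directions.
; Nearest-component search penalizes gear-to-gear pairs, and an overlap pass spawns collision-disabling links within a group.
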(fn RotateAroundAix
  (params (Rotate :type Rotator) (Aix :type Vector) (Angle :type Float%20%28double-precision%29))
  ;[0 0.4221 1] 将一个旋转值绕一个轴旋转一定角度   -  Rotate a rotate around aix
  (return (Math|Rotator|MakeRotationfromAxes (Math|Vector|RotateVectorAroundAxis (Math|Vector|GetForwardVector Rotate) Angle Aix) (Math|Vector|RotateVectorAroundAxis (Math|Vector|GetRightVector Rotate) Angle Aix) (Math|Vector|RotateVectorAroundAxis (Math|Vector|GetUpVector Rotate) Angle Aix))))

(fn GetCameraRotateandLocation
  (bind _returnvalue (Game|GetPlayerController 0))
  (bind _playercameramanager (Variables|/Script/Engine.PlayerController|GetPlayerCameraManager _returnvalue))
  (return (Camera|GetCameraLocation _playercameramanager) (Camera|GetCameraRotation _playercameramanager)))

(fn FindNearlyComponent
  (params (A :type Array%20of%20Scene%20Component%20Object%20References) (B :type Array%20of%20Scene%20Component%20Object%20References))
  (bind _distancearray (LocalVariables|GetDistanceArray))
  (bind (_indexofminvalue _minvalue) (Math|Float|MinOfFloatArray _distancearray))
  ;[1 0.3394 0] 弃用   Deprecate
  (for _array_element A
    (for _array_element_2 B
      (Utilities|Array|Add (LocalVariables|GetDistanceArray) (Math|Vector|VectorLength (- (Transformation|GetWorldLocation _array_element) (Transformation|GetWorldLocation _array_element_2))))
      (Utilities|Array|Add (LocalVariables|GetAGroup) _array_element)
      (Utilities|Array|Add (LocalVariables|GetBGroup) _array_element_2)))
  (return (Utilities|Array|Get(acopy) (LocalVariables|GetAGroup) _indexofminvalue) (Utilities|Array|Get(acopy) (LocalVariables|GetBGroup) _indexofminvalue) _minvalue))

(fn SetSimulatePhysics
  (params (Mesh :type Mesh%20Component%20Object%20Reference) (AssemblyComponent :type BPC%20Interaction%20Object%20Reference) (bSimulate :type Boolean))
  ;[0 0.4201 1] 当开启一个Mesh的模拟物理时，如果这个mesh的actor实现了 BPI_Simulate Physics的接口，则他通过接口去单独实现这个模拟物理，比如每个mesh模拟物理的规则可能不一样    When simulating physics for a Mesh by enabling its physics simulation, if the actor of this mesh implements the BPI_Simulate Physics interface, it individually implements the physics simulation through the interface. For example, each mesh may have different rules for physics simulation.
  (for _array_element (CallFunction|GetComponentConstraint AssemblyComponent Mesh false)
    (if bSimulate
      (if (Utilities|DoesObjectImplementInterface (Components|GetOwner _array_element) 0)
        (Class|BPIPhysicInteraction|CallTargetOverideSimulatePhysic(Message) (Components|GetOwner _array_element))
        (else
          (Physics|SetSimulatePhysics _array_element bSimulate)))
      (else
        (Physics|SetSimulatePhysics _array_element false)))))

(fn GetComponentConstraint
  (params (AssemblyComponent :type BPC%20Interaction%20Object%20Reference) (Mesh :type Mesh%20Component%20Object%20Reference) (GetInitConstraint :type Boolean))
  (bind (_return _find_) (CallFunction|GetRecordConstraint Mesh AssemblyComponent))
  (if GetInitConstraint
    (return (Actor|GetComponentsByClass (Components|GetOwner Mesh) "/Script/Engine.MeshComponent"))
    (elif _find_
      (return (Variables|/Game/BP/BasicActor/BP_RecordConstraint.BP_RecordConstraint_C|GetMeshGroup _return))
      (else
        (return (Utilities|Array|MakeArray Mesh))))))

(fn GetRecordConstraint
  (params (Component :type Mesh%20Component%20Object%20Reference) (AssemblyComponent :type BPC%20Interaction%20Object%20Reference))
  (bind _componenttags (Variables|/Script/Engine.ActorComponent|GetComponentTags Component))
  (bind _output (Utilities|Array|Get(acopy) _componenttags))
  (Utilities|IsValid Component
    (:Is%20Valid
      (if (Utilities|Array|IsValidIndex _componenttags)
        (return (.Value (Utilities|Map|Find (Variables|/Game/BP/BPC_Interaction.BPC_Interaction_C|GetConstraintRecorder AssemblyComponent) _output)) true _output)
        (else
          _)))
    (:Is%20Not%20Valid
      _))
  (return 0 false "None"))

(fn Calc2VectorCenter
  (params (A :type Vector) (B :type Vector) (Alpha :type Float%20%28double-precision%29))
  (return (Math|Vector|Normalize (+ (* A Alpha) (* B (- 1.0 Alpha))))))

(fn CalcMatrix
  (params (Transform :type Transform))
  (bind _returnvalue (Math|Vector|MakeVector 0.0 0.0 1.0))
  (bind _returnvalue_2 (Math|Vector|MakeVector 0.0 1.0 0.0))
  (bind _returnvalue_3 (Math|Vector|MakeVector 1.0 0.0 0.0))
  (bind _vgroup3 (LocalVariables|GetVGroup3))
  (bind _returnvalue_4 (CallFunction|Calc2VectorCenter _returnvalue_3 _returnvalue 0.5))
  (bind _returnvalue_5 (CallFunction|Calc2VectorCenter _returnvalue _returnvalue_2 0.5))
  (bind _returnvalue_6 (CallFunction|Calc2VectorCenter _returnvalue_3 _returnvalue_2 0.5))
  (bind _returnvalue_7 (CallFunction|Calc2VectorCenter _returnvalue _returnvalue_6 0.5))
  (bind _array (Utilities|Array|MakeArray _returnvalue_3 _returnvalue _returnvalue_2 _returnvalue_4 _returnvalue_5 _returnvalue_6 _returnvalue_7))
  (Utilities|FlowControl|Sequence
    (:then_0
      (LocalVariables|SetVGroup1 _array))
    (:then_1
      (for _array_element _array
        (Utilities|Array|AddUnique (LocalVariables|GetVGroup1) (* _array_element -1.0))))
    (:then_2
      (for _array_element_2 (LocalVariables|GetVGroup1)
        (Utilities|Array|AddUnique (LocalVariables|GetVGroup2) (Math|Vector|RotateVectorAroundAxis _array_element_2 9e+01 "0, 0,1.000000"))
        (Utilities|Array|AddUnique (LocalVariables|GetVGroup2) _array_element_2)))
    (:then_3
      (for _array_element_3 (LocalVariables|GetVGroup2)
        (Utilities|Array|AddUnique _vgroup3 (Math|Vector|RotateVectorAroundAxis _array_element_3 1.8e+02 "0, 0,1.000000"))
        (Utilities|Array|AddUnique _vgroup3 _array_element_3)))
    (:then_4
      (for _array_element_4 (LocalVariables|GetVGroup3)
        (Utilities|Array|Add (LocalVariables|GetVGroup4) (Math|Transform|TransformDirection Transform _array_element_4)))
      (return (LocalVariables|GetVGroup4)))))

(fn FindSnapRotate
  (params (Matrix :type Array%20of%20Vectors) (Rotate :type Rotator))
  (bind _newlocalvar_1 (LocalVariables|GetNewLocalVar_1))
  (bind _front90cache (LocalVariables|GetFront90Cache))
  (Utilities|FlowControl|Sequence
    (:then_0
      (Utilities|Array|Clear (LocalVariables|GetNewLocalVar_0))
      (for _array_element Matrix
        (Utilities|Array|Add (LocalVariables|GetNewLocalVar_0) (CallFunction|CalcAngle _array_element (Math|Vector|GetForwardVector Rotate))))
      (LocalVariables|SetFront (Utilities|Array|Get(acopy) Matrix (.IndexOfMinValue (Math|Float|MinOfFloatArray (LocalVariables|GetNewLocalVar_0))))))
    (:then_1
      (for _array_element_2 Matrix
        (if (Math|Float|InRange(Float) (CallFunction|CalcAngle _array_element_2 (LocalVariables|GetFront)) 89.0 91.0)
          (Utilities|Array|Add (LocalVariables|GetFront90Cache) _array_element_2))))
    (:then_2
      (for _array_element_3 _front90cache
        (for _array_element_4 _front90cache
          (if (Math|Float|InRange(Float) (CallFunction|CalcAngle _array_element_3 _array_element_4) 89.0 91.0)
            (Utilities|Array|Add _newlocalvar_1 (Math|Rotator|MakeRotationfromAxes (LocalVariables|GetFront) _array_element_4 _array_element_3))
            (Utilities|Array|Add _newlocalvar_1 (Math|Rotator|MakeRotationfromAxes (LocalVariables|GetFront) _array_element_3 _array_element_4))))))
    (:then_3
      (for _array_element_5 (LocalVariables|GetNewLocalVar_1)
        (Utilities|Array|Add (LocalVariables|GetNewLocalVar_2) (Class|KismetMathLibrary|QuatAngularDistance (Class|KismetMathLibrary|MatrixtoQuat (Math|Transform|ToMatrix(Transform) (Math|Transform|MakeTransform "0, 0, 0" _array_element_5 "1.000000,1.000000,1.000000"))) (Class|KismetMathLibrary|MatrixtoQuat (Math|Transform|ToMatrix(Transform) (Math|Transform|MakeTransform "0, 0, 0" Rotate "1.000000,1.000000,1.000000"))))))
      (return (Utilities|Array|Get(acopy) (LocalVariables|GetNewLocalVar_1) (.IndexOfMinValue (Math|Float|MinOfFloatArray (LocalVariables|GetNewLocalVar_2))))))))

(fn CalcAngle
  (params (A :type Vector) (B :type Vector))
  (return (Class|KismetMathLibrary|DegAcos (Math|Vector|DotProduct A B))))

(fn GetActorConstraint
  (params (AssemblyComponent :type BPC%20Interaction%20Object%20Reference) (Mesh :type Mesh%20Component%20Object%20Reference) (GetInitConstraint :type Boolean))
  (bind _returnvalue (Components|GetOwner Mesh))
  (bind (_return _find_) (CallFunction|GetRecordConstraint Mesh AssemblyComponent))
  (if GetInitConstraint
    (return (Utilities|Array|MakeArray _returnvalue))
    (elif _find_
      (return (Variables|/Game/BP/BasicActor/BP_RecordConstraint.BP_RecordConstraint_C|GetActors _return))
      (else
        (return (Utilities|Array|MakeArray _returnvalue))))))

(fn TransformTransform
  (params (A :type Transform%20%28by%20ref%29) (B :type Transform%20%28by%20ref%29))
  (bind (_location _rotation _scale) (Math|Transform|BreakTransform B))
  (return (Math|Transform|MakeTransform (Math|Transform|TransformLocation A _location) (Math|Transform|TransformRotation A _rotation) (* (.Scale (Math|Transform|BreakTransform A)) _scale))))

(fn GetLocalyAssemblyComponent
  (return (Actor|GetComponentbyClass (Game|GetPlayerCharacter 0) "/Game/BP/BPC_Interaction.BPC_Interaction_C")))

(fn DisableOverlapComponentCollision
  (params (Component :type Mesh%20Component%20Object%20Reference))
  (bind _returnvalue (CallFunction|GetLocalyAssemblyComponent))
  (bind _cachecomponent (LocalVariables|GetCacheComponent))
  (bind _cachecomponent_2 (LocalVariables|GetCacheComponent))
  (bind _cachecomponent_3 (LocalVariables|GetCacheComponent))
  (bind _cachecomponent_4 (LocalVariables|GetCacheComponent))
  (bind _return (CallFunction|GetRecordConstraint Component _returnvalue))
  (bind _meshgroup (Variables|/Game/BP/BasicActor/BP_RecordConstraint.BP_RecordConstraint_C|GetMeshGroup _return))
  (Utilities|FlowControl|Sequence
    (:then_0
      (Utilities|FlowControl|Sequence
        (:then_0
          (for _array_element (Variables|/Game/BP/BasicActor/BP_RecordConstraint.BP_RecordConstraint_C|GetGlueGroup _return)
            (Utilities|Array|Add _cachecomponent_2 (Utilities|Struct|MakeS_MeshComponent (Variables|/Game/BP/BasicActor/BP_Glue.BP_Glue_C|GetA _array_element) (Variables|/Game/BP/BasicActor/BP_Glue.BP_Glue_C|GetB _array_element)))
            (Utilities|Array|Add _cachecomponent_2 (Utilities|Struct|MakeS_MeshComponent (Variables|/Game/BP/BasicActor/BP_Glue.BP_Glue_C|GetB _array_element) (Variables|/Game/BP/BasicActor/BP_Glue.BP_Glue_C|GetA _array_element)))))
        (:then_1
          (for _array_element_2 (Variables|/Game/BP/BasicActor/BP_RecordConstraint.BP_RecordConstraint_C|GetDisableCollisionGroup _return)
            (Utilities|Array|Add _cachecomponent_3 (Utilities|Struct|MakeS_MeshComponent (Variables|/Game/BP/BasicActor/BP_DisableCollisionGlue.BP_DisableCollisionGlue_C|GetA _array_element_2) (Variables|/Game/BP/BasicActor/BP_DisableCollisionGlue.BP_DisableCollisionGlue_C|GetB _array_element_2)))
            (Utilities|Array|Add _cachecomponent_3 (Utilities|Struct|MakeS_MeshComponent (Variables|/Game/BP/BasicActor/BP_DisableCollisionGlue.BP_DisableCollisionGlue_C|GetB _array_element_2) (Variables|/Game/BP/BasicActor/BP_DisableCollisionGlue.BP_DisableCollisionGlue_C|GetA _array_element_2)))))))
    (:then_1
      (for _array_element_3 _meshgroup
        (Utilities|Map|Add (LocalVariables|GetCacheCollision) _array_element_3 (Collision|GetCollisionProfileName _array_element_3))
        (Collision|SetCollisionProfileName _array_element_3 "overlapall" true :!class /Script/Engine.PrimitiveComponent)))
    (:then_2
      (for _array_element_4 _meshgroup
        (Utilities|FlowControl|Sequence
          (:then_0
            (for _array_element_5 (Class|PrimitiveComponent|GetOverlappingComponents _array_element_4)
              (bind _asmesh_component (Utilities|Casting|CastToMeshComponent _array_element_5))
              (if (Math|Boolean|ANDBoolean (not (or (Utilities|Array|ContainsItem _cachecomponent_4 (Utilities|Struct|MakeS_MeshComponent _array_element_4 _asmesh_component)) (Utilities|Array|ContainsItem _cachecomponent_4 (Utilities|Struct|MakeS_MeshComponent _asmesh_component _array_element_4)))) (Utilities|Array|ContainsItem _meshgroup _asmesh_component) (not (== (Components|GetOwner _array_element_4) (Components|GetOwner _array_element_5))))
                (bind _returnvalue_2 (Default|SpawnDisableGlue (CallFunction|GetLocalyAssemblyComponent) _array_element_4 _asmesh_component))
                (Utilities|Array|Add (Variables|/Game/BP/BasicActor/BP_RecordConstraint.BP_RecordConstraint_C|GetDisableCollisionGroup _return) _returnvalue_2)
                (Utilities|Array|Add _cachecomponent (Utilities|Struct|MakeS_MeshComponent _array_element_4 _asmesh_component))
                (Utilities|Array|Add _cachecomponent (Utilities|Struct|MakeS_MeshComponent _asmesh_component _array_element_4)))))
          (:then_1
            (Collision|SetCollisionProfileName _array_element_4 (.Value (Utilities|Map|Find (LocalVariables|GetCacheCollision) _array_element_4)) true :!class /Script/Engine.PrimitiveComponent)))))))

(fn FindNearlyComponent2
  (params (A :type Array%20of%20Scene%20Component%20Object%20References) (B :type Array%20of%20Mesh%20Component%20Object%20References))
  (bind _distancearray (LocalVariables|GetDistanceArray))
  (bind (_indexofminvalue _minvalue) (Math|Float|MinOfFloatArray _distancearray))
  ;[0 0.2086 0.7552] 找出这两个输入的component数组里，距离最近的两个component   Find the two components with the closest distance among these two input component arrays.
  (for _array_element A
    (for _array_element_2 B
      (if (and (or (== (Utilities|GetClass (Components|GetOwner _array_element)) "/Game/LevelDesignAsset/Constain/BP_Gear.BP_Gear_C") (Utilities|ClassIsChildOf (Utilities|GetClass (Components|GetOwner _array_element)) "/Game/LevelDesignAsset/Constain/BP_Gear.BP_Gear_C")) (or (== (Utilities|GetClass (Components|GetOwner _array_element_2)) "/Game/LevelDesignAsset/Constain/BP_Gear.BP_Gear_C") (Utilities|ClassIsChildOf (Utilities|GetClass (Components|GetOwner _array_element_2)) "/Game/LevelDesignAsset/Constain/BP_Gear.BP_Gear_C")))
        ;[0 0.3217 1] 如果A和B都是齿轮，那么他们之间的距离增加一个数值，当齿轮靠近齿轮时，我不希望他们优先合并到对方身上，因为他们都要合并到墙上   If both A and B are gears, then their distance increases by a certain value. When gears approach each other, I do not want them to prioritize merging with each other, as they both need to merge onto the wall.
        (Utilities|Array|Add (LocalVariables|GetDistanceArray) (+ (.ReturnValue (Collision|GetClosestPointonCollision _array_element_2 (Transformation|GetWorldLocation _array_element) "None")) 1e+04))
        (else
          (Utilities|Array|Add (LocalVariables|GetDistanceArray) (.ReturnValue (Collision|GetClosestPointonCollision _array_element_2 (Transformation|GetWorldLocation _array_element) "None")))))
      (Utilities|Array|Add (LocalVariables|GetAGroup) _array_element)
      (Utilities|Array|Add (LocalVariables|GetBGroup) _array_element_2)
      (Utilities|Array|Add (LocalVariables|GetVector) (.OutPointOnBody (Collision|GetClosestPointonCollision _array_element_2 (Transformation|GetWorldLocation _array_element) "None")))))
  (return (Utilities|Array|Get(acopy) (LocalVariables|GetAGroup) _indexofminvalue) (Utilities|Array|Get(acopy) (LocalVariables|GetBGroup) _indexofminvalue) _minvalue (Utilities|Array|Get(acopy) (LocalVariables|GetVector) _indexofminvalue)))

(fn RegisterActor
  (params (Target :type Actor%20Object%20Reference))
  (LocalVariables|SetMeshComp (Actor|GetComponentsByClass Target "/Script/Engine.MeshComponent"))
  (bind _output_get (LocalVariables|SetAssemblyComponent (Actor|GetComponentbyClass (Game|GetPlayerCharacter 0) "/Game/BP/BPC_Interaction.BPC_Interaction_C")))
  (bind _key (Default|CreateKey (LocalVariables|GetAssemblyComponent)))
  (LocalVariables|SetKey _key)
  (bind _returnvalue (Game|ConstructObjectfromClass _output_get "/Game/BP/BasicActor/BP_RecordConstraint.BP_RecordConstraint_C" _output_get (LocalVariables|GetKey)))
  (LocalVariables|SetRecord _returnvalue)
  (Utilities|Map|Add (Variables|/Game/BP/BPC_Interaction.BPC_Interaction_C|GetConstraintRecorder (LocalVariables|GetAssemblyComponent)) (LocalVariables|GetKey) _returnvalue)
  (for _array_element (LocalVariables|GetMeshComp)
    (Utilities|Array|Add (Variables|/Script/Engine.ActorComponent|GetComponentTags _array_element) (LocalVariables|GetKey))
    (Utilities|Array|Add (Variables|/Game/BP/BasicActor/BP_RecordConstraint.BP_RecordConstraint_C|GetMeshGroup _returnvalue) _array_element))
  (Utilities|Array|AddUnique (Variables|/Game/BP/BasicActor/BP_RecordConstraint.BP_RecordConstraint_C|GetActors _returnvalue) Target))