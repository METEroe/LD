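; BP_PickUps is a pickup actor that takes its mesh from a data table row and highlights itself when detected.
; The construction script looks up the row in PickUpsCheck and applies its mesh, while AddType sets that struct.
; Detected spawns a collision-free duplicate mesh at the same location, using a highlight material with color and range parameters.
; NotDetected destroys that overlay component.
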(event Custom|Show%20HighLight
  (for _index (range 0 (- (Utilities|Array|Length (Rendering|Material|GetMaterials (Variables|Default|GetHighLightMesh))) 1))
    (Rendering|Material|SetMaterial (Variables|Default|GetHighLightMesh) _index "/Game/BP/PickUps/MI_HighLight.MI_HighLight")
    (Rendering|Material|SetVectorParameterValueonMaterials (Variables|Default|GetHighLightMesh) "HighLightColor" (Variables|Default|GetHighLightColor))
    (Rendering|Material|SetScalarParameterValueonMaterials (Variables|Default|GetHighLightMesh) "HighLightRange" (Variables|Default|GetHighLightRange))))

(event Custom|Add%20Type
  (params (PickUpsCheck :type S%20Pickup%20Attribute%20Structure))
  (Variables|Default|SetPickUpsCheck PickUpsCheck))

(event EventDetected
  (Variables|Default|GetHighLightMesh
    (:then)
    (:else
      (bind _returnvalue (AddComponent|AddStaticMeshComponent false))
      (bind _output_get (Variables|Default|SetHighLightMesh _returnvalue))
      (Components|StaticMesh|SetStaticMesh _output_get (Variables|Default|GetPickup%20Mesh))
      (Transformation|SetWorldLocation (Variables|Default|GetHighLightMesh) (Transformation|GetWorldLocation (Variables|Default|GetStaticMesh)) false false)
      (Collision|SetCollisionEnabled (Variables|Default|GetHighLightMesh) "NoCollision")
      (CallFunction|ShowHighLight))))

(event EventNotDetected
  (bind _highlightmesh (Variables|Default|GetHighLightMesh)
    (:then
      (Components|DestroyComponent _highlightmesh))
    (:else)))

(fn ConstructionScript
  (bind _pickupscheck (Variables|Default|GetPickUpsCheck))
  (bind _returnvalue (Utilities|GetDataTableRow (.datatable (.pickupstable _pickupscheck)) (.rowname (.pickupstable _pickupscheck)))
    (:then
      (bind _output_get (Variables|Default|SetPickup%20Mesh (.Mesh (Utilities|Struct|BreakS_PickUpList _returnvalue))))
      (Components|StaticMesh|SetStaticMesh (Variables|Default|GetStaticMesh) _output_get))))