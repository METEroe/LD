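; Records a group of assembled meshes and glue constraints and packs them into save data for a player "blueprint system".
; AddComponent clears the mesh's record info, tags it with a key and registers it and its owner; RemoveComponent is empty.
; MakeSaveData stores actor classes, component transforms and glue endpoints with a screenshot path.
; Actor and glue transforms are relative to the supplied grab transform, component transforms to their owning actor.
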(event Custom|AddComponent
  (params (Component :type Mesh%20Component%20Object%20Reference))
  (Utilities|FlowControl|Sequence
    (:then_0
      (Default|ClearRecordInfo (Variables|Default|GetAssemblyComponent) Component)
      (Utilities|Array|Add (Variables|/Script/Engine.ActorComponent|GetComponentTags Component) (Variables|Default|GetKey)))
    (:then_1
      (Utilities|Array|AddUnique (Variables|Default|GetMeshGroup) Component)
      (Utilities|Array|AddUnique (Variables|Default|GetActors) (Components|GetOwner Component)))))

(event Custom|RemoveComponent)

(fn CalcIgornActors
  (for _array_element (Variables|Default|GetMeshGroup)
    (Utilities|Array|AddUnique (Variables|Default|GetActors) (Components|GetOwner _array_element))))

(fn MakeSaveData
  (params (Name :type Name) (GrapTransform :type Transform))
  (bind _returnvalue (Utilities|String|ToString(Name) Name))
  ;[0 0.5226 1] Create a "blueprint system" save data  记录数据，准备存档
  (LocalVariables|SetBaseTransform GrapTransform)
  (Utilities|FlowControl|Sequence
    (:then_0
      (for _array_element (Variables|Default|GetActors)
        (for _array_element_2 (Actor|GetComponentsByClass _array_element "/Script/Engine.MeshComponent")
          (Utilities|Map|Add (LocalVariables|GetComponentCache) (Utilities|GetObjectName _array_element_2) (Math|Transform|MakeRelativeTransform (Transformation|GetWorldTransform _array_element_2) (Transformation|GetActorTransform _array_element)))
          (Utilities|Array|Add (LocalVariables|GetCacheComponents) _array_element_2))
        (Utilities|Array|Add (LocalVariables|GetActorTransform) (Utilities|Struct|MakeS_PhysicsActorInfo (Math|Transform|MakeRelativeTransform (Transformation|GetActorTransform _array_element) (LocalVariables|GetBaseTransform)) (Utilities|GetClass _array_element) (LocalVariables|GetComponentCache)))
        (Utilities|Array|Add (LocalVariables|GetActorClass) (Utilities|GetClass _array_element))
        (Utilities|Map|Clear (LocalVariables|GetComponentCache))))
    (:then_1
      (for _array_element_3 (Variables|Default|GetGlueGroup)
        (Utilities|Array|Add (LocalVariables|GetGlueInfo) (Utilities|Struct|MakeS_GlueInfo (Math|Transform|MakeRelativeTransform (Transformation|GetActorTransform _array_element_3) (LocalVariables|GetBaseTransform)) (Utilities|GetObjectName (Variables|/Game/BP/BasicActor/BP_Glue.BP_Glue_C|GetA _array_element_3)) (Utilities|GetObjectName (Variables|/Game/BP/BasicActor/BP_Glue.BP_Glue_C|GetB _array_element_3)) (Math|Transform|TransformLocation (LocalVariables|GetBaseTransform) (Variables|/Game/BP/BasicActor/BP_Glue.BP_Glue_C|GetPointA _array_element_3)) (Math|Transform|TransformLocation (LocalVariables|GetBaseTransform) (Variables|/Game/BP/BasicActor/BP_Glue.BP_Glue_C|GetPointB _array_element_3)) (Variables|/Game/BP/BasicActor/BP_Glue.BP_Glue_C|GetBoneA _array_element_3) (Variables|/Game/BP/BasicActor/BP_Glue.BP_Glue_C|GetBoneB _array_element_3) (Math|Transform|MakeRelativeTransform (Transformation|GetActorTransform (Components|GetOwner (Variables|/Game/BP/BasicActor/BP_Glue.BP_Glue_C|GetA _array_element_3))) (Transformation|GetActorTransform _array_element_3)) (Math|Transform|MakeRelativeTransform (Transformation|GetActorTransform (Components|GetOwner (Variables|/Game/BP/BasicActor/BP_Glue.BP_Glue_C|GetB _array_element_3))) (Transformation|GetActorTransform _array_element_3)) (Utilities|GetClass (Components|GetOwner (Variables|/Game/BP/BasicActor/BP_Glue.BP_Glue_C|GetA _array_element_3))) (Utilities|GetClass (Components|GetOwner (Variables|/Game/BP/BasicActor/BP_Glue.BP_Glue_C|GetB _array_element_3)))))))
    (:then_2
      (return (Utilities|Struct|MakeS_SavingData _returnvalue (Utilities|String|Append "Saved\\Screenshots\\WindowsEditor\\" _returnvalue ".png") (LocalVariables|GetBaseTransform) (LocalVariables|GetActorTransform) (LocalVariables|GetGlueInfo))))))