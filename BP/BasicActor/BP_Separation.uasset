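; BP_Separation regroups the glued actors connected to a given actor into their own assembly record under a new key.
; Calc creates a BP_RecordConstraint in the AssemblyComponent, then recursively searches glue links, consuming each match to collect connected actors.
; It tags their mesh components with the key, stores actors, meshes and glue in the record, and refreshes physics and overlap collision through the first mesh.
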(event Custom|Calc
  (bind _assemblycomponent (Variables|Default|GetAssemblyComponent))
  (bind _component (Variables|Default|GetComponent))
  (bind _assemblycomponent_2 (Variables|Default|GetAssemblyComponent))
  (bind _output (Utilities|Array|Get(acopy) _component))
  (Utilities|FlowControl|Sequence
    (:then_0
      (bind _key (Default|CreateKey _assemblycomponent))
      (bind _returnvalue (Game|ConstructObjectfromClass _assemblycomponent "/Game/BP/BasicActor/BP_RecordConstraint.BP_RecordConstraint_C" _assemblycomponent _key))
      (bind _output_get (Variables|Default|SetRec _returnvalue))
      (Utilities|Map|Add (Variables|/Game/BP/BPC_Interaction.BPC_Interaction_C|GetConstraintRecorder _assemblycomponent) _key _output_get)
      (Variables|Default|SetKey _key))
    (:then_1
      (bind _return (CallFunction|IterativeSearch (Utilities|Array|MakeArray (Variables|Default|GetActor)) (Variables|Default|GetActor) (Variables|Default|GetGlueGroup)))
      (Variables|Default|SetActors _return)
      (for _array_element _return
        (for _array_element_2 (Actor|GetComponentsByClass _array_element "/Script/Engine.MeshComponent")
          (Utilities|Array|SetArrayElem (Variables|/Script/Engine.ActorComponent|GetComponentTags _array_element_2) 0 (Variables|Default|GetKey))
          (Utilities|Array|Add (Variables|Default|GetComponent) _array_element_2))))
    (:then_2
      (Variables|/Game/BP/BasicActor/BP_RecordConstraint.BP_RecordConstraint_C|SetActors (Variables|Default|GetRec) (Variables|Default|GetActors))
      (Variables|/Game/BP/BasicActor/BP_RecordConstraint.BP_RecordConstraint_C|SetMeshGroup (Variables|Default|GetRec) (Variables|Default|GetComponent))
      (Variables|/Game/BP/BasicActor/BP_RecordConstraint.BP_RecordConstraint_C|SetGlueGroup (Variables|Default|GetRec) (Variables|Default|GetGlueResult)))
    (:then_3
      (Default|SimulatePhysicsAssembly _assemblycomponent_2 _output false)
      (Default|DisableOverlapCollision _assemblycomponent_2 _output)
      (Default|SimulatePhysicsAssembly _assemblycomponent_2 _output true))))

(fn IterativeSearch
  (params (ActorCache :type Array%20of%20Actor%20Object%20References) (curActor :type Actor%20Object%20Reference) (Glue :type Array%20of%20BP%20Glue%20Object%20References))
  (LocalVariables|SetGlue_ Glue)
  (LocalVariables|SetActor_ ActorCache)
  (bind _array_element (Utilities|Array|ForEachLoopwithBreak Glue)
    (:LoopBody
      (if (or (== (Components|GetOwner (Variables|/Game/BP/BasicActor/BP_Glue.BP_Glue_C|GetA _array_element)) curActor) (== (Components|GetOwner (Variables|/Game/BP/BasicActor/BP_Glue.BP_Glue_C|GetB _array_element)) curActor))
        (Utilities|Array|Add (Variables|Default|GetGlueResult) _array_element)
        (LocalVariables|SetFind? true)
        (Utilities|Array|RemoveItem (LocalVariables|GetGlue_) _array_element)
        (Utilities|FlowControl|Sequence
          (:then_0
            (if (== (Components|GetOwner (Variables|/Game/BP/BasicActor/BP_Glue.BP_Glue_C|GetA _array_element)) curActor)
              (Utilities|Array|Add (LocalVariables|GetActor_) (Components|GetOwner (Variables|/Game/BP/BasicActor/BP_Glue.BP_Glue_C|GetB _array_element)))
              (LocalVariables|SetActorToCheckNextTime (Components|GetOwner (Variables|/Game/BP/BasicActor/BP_Glue.BP_Glue_C|GetB _array_element)))
              (else
                (Utilities|Array|Add (LocalVariables|GetActor_) (Components|GetOwner (Variables|/Game/BP/BasicActor/BP_Glue.BP_Glue_C|GetA _array_element)))
                (LocalVariables|SetActorToCheckNextTime (Components|GetOwner (Variables|/Game/BP/BasicActor/BP_Glue.BP_Glue_C|GetA _array_element))))))
          (:then_1
            (bind _return (CallFunction|IterativeSearch (LocalVariables|GetActor_) (LocalVariables|GetActorToCheckNextTime) (LocalVariables|GetGlue_)))
            (LocalVariables|SetActor_ _return)))))
    (:Completed
      (return (LocalVariables|GetActor_)))))