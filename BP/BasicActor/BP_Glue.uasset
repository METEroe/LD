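; Glue actor that joins two components in an assembly system with a physics constraint, freeing angular limits if either is a skeletal mesh.
; StartCombine pauses physics, then a timeline pulls both contact points to their midpoint, snapping A's rotation to B (gears excepted) and carrying constrained parts along.
; It then constrains the pair, attaches to A, records the link and resumes simulation.
; CombineFromSaveData restores the constraint and attachment without animation.
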(event Custom|StartCombine
  (bind _pointa (Variables|Default|GetPointA))
  (bind _pointb (Variables|Default|GetPointB))
  (bind _a (Variables|Default|GetA))
  (bind _a_2 (Variables|Default|GetA))
  (bind _b (Variables|Default|GetB))
  (bind _a_3 (Variables|Default|GetA))
  (bind _returnvalue (Utilities|GetClass _a))
  (bind _returnvalue_2 (* _pointb 0.5))
  (bind _returnvalue_3 (* _pointa 0.5))
  (bind _returnvalue_4 (+ _returnvalue_3 _returnvalue_2))
  (Utilities|FlowControl|Sequence
    (:then_1
      (CallFunction|SetSimulatePhysics (Variables|Default|GetA) (Variables|Default|GetAssemblySystem) false)
      (CallFunction|SetSimulatePhysics (Variables|Default|GetB) (Variables|Default|GetAssemblySystem) false))
    (:then_2
      (bind _output_get (Variables|Default|SetSelfInitLocation (Transformation|GetWorldLocation (Variables|Default|GetA))))
      (bind _output_get_2 (Variables|Default|SetOtherInitLocation (Transformation|GetWorldLocation (Variables|Default|GetB))))
      (Variables|Default|SetNewSelfLocation (+ _output_get (- _returnvalue_4 _pointa)))
      (Variables|Default|SetNewOtherLocation (+ (- _returnvalue_4 _pointb) _output_get_2))
      ;[1 1 1] Rotate Snap
      (if (or (== _returnvalue "/Game/LevelDesignAsset/Constain/BP_Gear.BP_Gear_C") (Utilities|ClassIsChildOf _returnvalue "/Game/LevelDesignAsset/Constain/BP_Gear.BP_Gear_C"))
        (Variables|Default|SetTargetRotate (Transformation|GetWorldRotation (Variables|Default|GetA)))
        (else
          (bind _vectormatrix (CallFunction|CalcMatrix (Transformation|GetWorldTransform (Variables|Default|GetB))))
          (bind _output (CallFunction|FindSnapRotate _vectormatrix (Transformation|GetWorldRotation (Variables|Default|GetA))))
          (Variables|Default|SetTargetRotate _output)
          (Variables|Default|SetInitRotate (Transformation|GetWorldRotation (Variables|Default|GetA)))
          (Utilities|FlowControl|Sequence
            (:then_0
              (bind _output_get_3 (Variables|Default|SetReturn (CallFunction|GetComponentConstraint (Variables|Default|GetAssemblySystem) (Variables|Default|GetA) false)))
              (for _array_element _output_get_3
                (Utilities|Array|Add (Variables|Default|GetATrans) (Math|Transform|MakeRelativeTransform (Transformation|GetWorldTransform _array_element) (Transformation|GetWorldTransform (Variables|Default|GetA))))))
            (:then_1
              (bind _output_get_4 (Variables|Default|SetReturn_0 (CallFunction|GetComponentConstraint (Variables|Default|GetAssemblySystem) (Variables|Default|GetB) false)))
              (for _array_element_2 _output_get_4
                (Utilities|Array|Add (Variables|Default|GetBTrans) (Math|Transform|MakeRelativeTransform (Transformation|GetWorldTransform _array_element_2) (Transformation|GetWorldTransform (Variables|Default|GetB))))))))))
    (:then_3
      ;[1 1 1] Combine Animation
      (bind _newtrack_0 (Timeline|Timeline_0 PlayFromStart)
        (:Update
          (Transformation|SetWorldLocation (Variables|Default|GetB) (Math|Vector|Lerp(Vector) (Variables|Default|GetOtherInitLocation) (Variables|Default|GetNewOtherLocation) _newtrack_0) false true)
          (Transformation|SetWorldLocation _a_2 (Math|Vector|Lerp(Vector) (Variables|Default|GetSelfInitLocation) (Variables|Default|GetNewSelfLocation) _newtrack_0) false true)
          (Transformation|SetWorldRotation _a_2 (Math|Rotator|Lerp(Rotator) (Variables|Default|GetInitRotate) (Variables|Default|GetTargetRotate) _newtrack_0 true) false false)
          (Utilities|FlowControl|Sequence
            (:then_0
              (for (_array_element_3 _array_index) (Variables|Default|GetReturn)
                (if (!= _array_element_3 _a_3)
                  (Transformation|SetWorldTransform _array_element_3 (CallFunction|TransformTransform (Transformation|GetWorldTransform _a_3) (Utilities|Array|Get(acopy) (Variables|Default|GetATrans) _array_index)) false false))))
            (:then_1
              (for (_array_element_4 _array_index_2) (Variables|Default|GetReturn_0)
                (if (!= _array_element_4 _b)
                  (Transformation|SetWorldTransform _array_element_4 (CallFunction|TransformTransform (Transformation|GetWorldTransform _b) (Utilities|Array|Get(acopy) (Variables|Default|GetBTrans) _array_index_2)) false false))))))
        (:Finished
          (Utilities|FlowControl|Sequence
            (:then_0
              (CallFunction|CheckIsSkeletonMesh))
            (:then_1
              (Class|PhysicsConstraintComponent|SetConstrainedComponents (Variables|Default|GetPhysicsConstraint) (Variables|Default|GetA) (Variables|Default|GetBoneA) (Variables|Default|GetB) (Variables|Default|GetBoneB)))
            (:then_3
              (Transformation|AttachComponentToComponent (Variables|Default|GetA) (Variables|Default|GetBoneA) "KeepWorld" "KeepWorld" "KeepWorld" true)
              (Default|AddRecordConstraintInfo (Variables|Default|GetAssemblySystem) (Variables|Default|GetA) (Variables|Default|GetB) self)
              (Utilities|FlowControl|Sequence
                (:then_0
                  (CallFunction|DisableOverlapComponentCollision (Variables|Default|GetA)))
                (:then_1
                  (Utilities|Array|Clear (Variables|Default|GetATrans))
                  (Utilities|Array|Clear (Variables|Default|GetBTrans))
                  (CallFunction|SetSimulatePhysics (Variables|Default|GetA) (Variables|Default|GetAssemblySystem) true))))))))))

(event Custom|CombineFromSaveData
  (Utilities|FlowControl|Sequence
    (:then_0
      (CallFunction|CheckIsSkeletonMesh))
    (:then_2
      (Class|PhysicsConstraintComponent|SetConstrainedComponents (Variables|Default|GetPhysicsConstraint) (Variables|Default|GetA) (Variables|Default|GetBoneA) (Variables|Default|GetB) (Variables|Default|GetBoneB))
      (Transformation|AttachComponentToComponent (Variables|Default|GetA) (Variables|Default|GetBoneA) "KeepWorld" "KeepWorld" "KeepWorld" true))))

(event Custom|CheckIsSkeletonMesh
  (bind _physicsconstraint (Variables|Default|GetPhysicsConstraint))
  (if (or (.bSuccess (Utilities|Casting|CastToSkeletalMeshComponent (Variables|Default|GetA))) (.bSuccess (Utilities|Casting|CastToSkeletalMeshComponent (Variables|Default|GetB))))
    (Class|PhysicsConstraintComponent|SetAngularSwing1Limit _physicsconstraint "ACM_Free" 0.0)
    (Class|PhysicsConstraintComponent|SetAngularTwistLimit _physicsconstraint "ACM_Free" 0.0)
    (Class|PhysicsConstraintComponent|SetAngularSwing2Limit _physicsconstraint "ACM_Free" 0.0)))

(fn ConstructionScript)