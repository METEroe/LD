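; BP_BulletButton is a short-lived actor, named as a bullet, that sends interaction messages to what it touches and expires two seconds after spawning.
; When its sphere overlaps a mesh component, it looks up that mesh's constraint record using the local assembly component.
; A valid record passes the interact message to all its actors and destroys the bullet.
; Otherwise, only the mesh's owner receives the message and the bullet persists.
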(event OnComponentBeginOverlap(Sphere1)
  (params (OverlappedComponent :type Primitive%20Component%20Object%20Reference) (OtherActor :type Actor%20Object%20Reference) (OtherComp :type Primitive%20Component%20Object%20Reference) (OtherBodyIndex :type Integer) (bFromSweep :type Boolean) (SweepResult :type Hit%20Result%20Structure%20%28by%20ref%29))
  (bind _asmesh_component (Utilities|Casting|CastToMeshComponent OtherComp))
  (Utilities|IsValid (.Return (CallFunction|GetRecordConstraint _asmesh_component (CallFunction|GetLocalyAssemblyComponent)))
    (:Is%20Valid
      (for _array_element (Variables|/Game/BP/BasicActor/BP_RecordConstraint.BP_RecordConstraint_C|GetActors (.Return (CallFunction|GetRecordConstraint _asmesh_component (CallFunction|GetLocalyAssemblyComponent))))
        (Class|BPIInteraction|InteracttoTarget(Message) _array_element "NewEnumerator0"))
      (Actor|DestroyActor))
    (:Is%20Not%20Valid
      (Class|BPIInteraction|InteracttoTarget(Message) (Components|GetOwner _asmesh_component) "NewEnumerator0"))))

(event EventBeginPlay
  (Utilities|FlowControl|Delay 2.0)
  (Actor|DestroyActor))

(event Collision|EventActorBeginOverlap
  (params (OtherActor :type Actor%20Object%20Reference)))

(event EventTick
  (params (DeltaSeconds :type Float%20%28single-precision%29)))

(fn ConstructionScript)