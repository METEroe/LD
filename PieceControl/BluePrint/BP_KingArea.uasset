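; BP_KingArea is a box trigger area that records whether an overlapping control piece has its pick-up flag set.
; The construction script sizes the box from the InBoxExtent variable.
; On begin overlap it casts the other actor to BP_ControlPiece and sets Pickup to 1 or 0 from that piece's PickUpFlag.
; Pickup is never reset on end overlap and is not read within this Blueprint.
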(event OnComponentBeginOverlap(Box)
  (params (OverlappedComponent :type Primitive%20Component%20Object%20Reference) (OtherActor :type Actor%20Object%20Reference) (OtherComp :type Primitive%20Component%20Object%20Reference) (OtherBodyIndex :type Integer) (bFromSweep :type Boolean) (SweepResult :type Hit%20Result%20Structure%20%28by%20ref%29))
  (bind _asbp_control_piece (Utilities|Casting|CastToBP_ControlPiece OtherActor))
  (bind _output_get (Variables|Default|SetAs%20BP%20Control%20Piece _asbp_control_piece))
  (if (Variables|/Game/PieceControl/BluePrint/BP_ControlPiece.BP_ControlPiece_C|GetPickUpFlag _output_get)
    (Variables|Default|SetPickup 1)
    (else
      (Variables|Default|SetPickup 0))))

(fn ConstructionScript
  (Variables|Default|SetIn%20Box%20Extent (Variables|Default|GetIn%20Box%20Extent))
  (Components|Box|SetBoxExtent (Variables|Default|GetBox) (Variables|Default|GetIn%20Box%20Extent) true))