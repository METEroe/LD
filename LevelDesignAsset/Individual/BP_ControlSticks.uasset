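; BP_ControlSticks is an interactable driving station that seats the player and steers the physics assembly it is constrained to.
; Interacting toggles driving, attaching or releasing the player and switching collision and movement.
; While driven, Tick applies angular impulses that right the stick mesh.
; Drive input reaches recorded assembly actors through an interface, or as angular impulses whose pitch and roll fade as the sticks tilt.
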(event OnComponentBeginOverlap(Sphere)
  (params (OverlappedComponent :type Primitive%20Component%20Object%20Reference) (OtherActor :type Actor%20Object%20Reference) (OtherComp :type Primitive%20Component%20Object%20Reference) (OtherBodyIndex :type Integer) (bFromSweep :type Boolean) (SweepResult :type Hit%20Result%20Structure%20%28by%20ref%29))
  (Class|BPICharacter|AddtoInteractRange(Message) OtherActor self))

(event OnComponentEndOverlap(Sphere)
  (params (OverlappedComponent :type Primitive%20Component%20Object%20Reference) (OtherActor :type Actor%20Object%20Reference) (OtherComp :type Primitive%20Component%20Object%20Reference) (OtherBodyIndex :type Integer))
  (Class|BPICharacter|RemovefromInteractRange(Message) OtherActor self))

(event EventBeginPlay)

(event Collision|EventActorBeginOverlap
  (params (OtherActor :type Actor%20Object%20Reference)))

(event EventTick
  (params (DeltaSeconds :type Float%20%28single-precision%29))
  (bind _returnvalue (Math|Vector|MakeVector 0.0 0.0 1.0))
  (bind _staticmesh (Variables|Default|GetStaticMesh))
  (bind _returnvalue_2 (Transformation|GetWorldRotation _staticmesh))
  (bind _returnvalue_3 (Math|Vector|GetUpVector _returnvalue_2))
  (if (Variables|Default|GetIs%20In%20Drive)
    (Class|PrimitiveComponent|AddAngularImpulseinDegrees _staticmesh (* (Math|Vector|CrossProduct _returnvalue_3 _returnvalue) (* (Class|KismetMathLibrary|DegAcos (Math|Vector|DotProduct _returnvalue_3 _returnvalue)) 1.2e+05)) "None" false)))

(event EventDriveTarget
  (params (Axis :type Vector%202D%20Structure))
  (bind _returnvalue (Math|Vector|MakeVector 0.0 0.0 1.0))
  (bind _returnvalue_2 (Game|GetPlayerCharacter 0))
  (bind (_x _y) (Math|Vector2D|BreakVector2D Axis))
  (bind _returnvalue_3 (Utilities|Time|GetWorldDeltaSeconds))
  (bind _staticmesh (Variables|Default|GetStaticMesh))
  (bind _staticmesh_2 (Variables|Default|GetStaticMesh))
  (bind _staticmesh_3 (Variables|Default|GetStaticMesh))
  (bind _returnvalue_4 (Transformation|GetWorldRotation _staticmesh_2))
  (bind _returnvalue_5 (Actor|GetComponentbyClass _returnvalue_2 "/Game/BP/BPC_Interaction.BPC_Interaction_C"))
  (bind _returnvalue_6 (* _returnvalue_3 1.2e+02))
  (bind _returnvalue_7 (Math|Vector|GetUpVector _returnvalue_4))
  (bind _return (CallFunction|GetRecordConstraint _staticmesh_3 _returnvalue_5))
  (bind _returnvalue_8 (* 1.2e+04 _returnvalue_6))
  (bind _returnvalue_9 (Math|Vector|DotProduct _returnvalue_7 _returnvalue))
  (bind _returnvalue_10 (Class|KismetMathLibrary|DegAcos _returnvalue_9))
  (bind _returnvalue_11 (Math|Float|MapRangeClamped _returnvalue_10 0.0 35.0 _returnvalue_8 0.0))
  (Utilities|IsValid _return
    (:Is%20Valid
      (for _array_element (Variables|/Game/BP/BasicActor/BP_RecordConstraint.BP_RecordConstraint_C|GetActors _return)
        (if (Utilities|DoesObjectImplementInterface _array_element 0)
          (Class|BPIPhysicInteraction|ControlTarget(Message) _array_element Axis self)
          (else
            (Class|PrimitiveComponent|AddAngularImpulseinRadians (Actor|GetComponentbyClass _array_element "/Script/Engine.MeshComponent") (+ (* (Math|Vector|GetRightVector _staticmesh) (* _y _returnvalue_11 -1.0)) (* (Math|Vector|GetForwardVector _staticmesh) (* _x _returnvalue_11 -1.0)) (* (Math|Vector|GetUpVector _staticmesh) (* _y 1.2e+04 (* (Utilities|Time|GetWorldDeltaSeconds) 1.2e+02)))) "None" false)))))))

(event EventInteracttoTarget
  (params (Input%20Type :type E_InteractType%20Enum :default "NewEnumerator0"))
  (bind _returnvalue (Game|GetPlayerCharacter 0))
  (bind _returnvalue_2 (Game|GetPlayerCharacter 0))
  (bind _returnvalue_3 (Game|GetPlayerCharacter 0))
  (bind _returnvalue_4 (Game|GetPlayerCharacter 0))
  (switch Utilities|FlowControl|Switch|SwitchonE_InteractType Input%20Type
    (:NewEnumerator1
      (if (Variables|Default|GetIs%20In%20Drive)
        (Variables|Default|SetIs%20In%20Drive false)
        (Transformation|SetActorRelativeLocation _returnvalue_3 "0,300.000000,200.000000")
        (Transformation|DetachFromActor _returnvalue_3 "KeepWorld" "KeepWorld" "KeepWorld")
        (Collision|SetCollisionEnabled (Variables|/Script/Engine.Character|GetCapsuleComponent _returnvalue_3) "QueryAndPhysics")
        (Transformation|SetActorRotation _returnvalue_3 (Math|Rotator|MakeRotator 0.0 0.0 (.yaw (Transformation|GetActorRotation _returnvalue_3))))
        (Variables|/Game/BP/BPC_Interaction.BPC_Interaction_C|SetInteractionActor (Actor|GetComponentbyClass _returnvalue_4 "/Game/BP/BPC_Interaction.BPC_Interaction_C") 0)
        (Pawn|Components|CharacterMovement|SetMovementMode (Variables|/Script/Engine.Character|GetCharacterMovement _returnvalue_4) "MOVE_Falling" 0)
        (else
          (Variables|Default|SetIs%20In%20Drive true)
          (Transformation|AttachComponentToComponent _returnvalue (Variables|Default|GetStaticMesh) "None" "SnapToTarget" "SnapToTarget" "KeepWorld" true)
          (Transformation|SetActorRelativeRotation _returnvalue "0,90.000000, 0")
          (Transformation|SetActorRelativeLocation _returnvalue "0, 0,95.000000")
          (Collision|SetCollisionEnabled (Variables|/Script/Engine.Character|GetCapsuleComponent _returnvalue) "NoCollision")
          (Variables|/Game/BP/BPC_Interaction.BPC_Interaction_C|SetInteractionActor (Actor|GetComponentbyClass _returnvalue_2 "/Game/BP/BPC_Interaction.BPC_Interaction_C") self)
          (Pawn|Components|CharacterMovement|SetMovementMode (Variables|/Script/Engine.Character|GetCharacterMovement _returnvalue_2) "MOVE_None" 0))))))

(fn ConstructionScript)