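; BP_Propeller is a physics-driven propeller for level design that turns its own spin into thrust.
; Each tick, while the mesh simulates physics, it converts angular velocity into local space and applies force along the mesh's up vector, scaled by the Z spin.
; The Invert flag reverses the thrust direction and swaps the mesh material in the construction script to mark the variant.
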(event EventBeginPlay
  (|CallParentFunction)
  (Utilities|FlowControl|Delay 2.0))

(event Collision|EventActorBeginOverlap
  (params (OtherActor :type Actor%20Object%20Reference)))

(event EventTick
  (params (DeltaSeconds :type Float%20%28single-precision%29))
  (bind _staticmesh (Variables|Default|GetStaticMesh))
  (Utilities|FlowControl|Sequence
    (:then_0
      (if (Physics|IsSimulatingPhysics (Variables|Default|GetStaticMesh) "None")
        (Physics|AddForce (Variables|Default|GetStaticMesh) (* (Math|Vector|GetUpVector _staticmesh) (* (.Z (Math|Vector|BreakVector (Math|Transform|InverseTransformDirection (Transformation|GetWorldTransform _staticmesh) (Class|PrimitiveComponent|GetPhysicsAngularVelocityinRadians _staticmesh "None")))) 1.3e+03 (select (Variables|Default|GetInvert) -1.0 1.0))) "None" false)))))

(event EventControlTarget
  (params (Axis :type Vector%202D%20Structure) (ControlActor :type Actor%20Object%20Reference)))

(fn ConstructionScript
  (|CallParentFunction)
  (if (Variables|Default|GetInvert)
    (Rendering|Material|SetMaterial (Variables|Default|GetStaticMesh) 0 "/Game/CommonAsset/Materials/MI_LDGrid_Local_Inst_2.MI_LDGrid_Local_Inst_2")))