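; Physics-driven wheel actor that Interact toggles on and off and a controlling actor can drive.
; While on and simulating, Tick applies curve-based angular impulses to StaticMesh and reversed ones to Cube2, both keyed on the wheel's local X spin speed.
; ControlTarget adds stick-driven impulses along the controller's axes: X scaled by a second speed curve, Y by the wheel's lateral offset from the controller.
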(event EventBeginPlay
  (|CallParentFunction))

(event Collision|EventActorBeginOverlap
  (params (OtherActor :type Actor%20Object%20Reference)))

(event EventTick
  (params (DeltaSeconds :type Float%20%28single-precision%29))
  (bind _x (CallFunction|WheelRotateSpeed))
  (bind _touquecurve (Variables|Default|GetTouqueCurve))
  (bind _cube2 (Variables|Default|GetCube2))
  (|CallParentFunction DeltaSeconds)
  (if (and (Variables|Default|GetON) (Physics|IsSimulatingPhysics (Variables|Default|GetStaticMesh) "None"))
    (Class|PrimitiveComponent|AddAngularImpulseinRadians (Variables|Default|GetStaticMesh) (* (Transformation|GetActorForwardVector) (* (Math|Curves|GetFloatValue _touquecurve _x) 0.65)) "None" false)
    (Class|PrimitiveComponent|AddAngularImpulseinRadians _cube2 (* (Math|Vector|GetForwardVector _cube2) (* (Math|Curves|GetFloatValue _touquecurve (- 1e+03 _x)) -1.0)) "None" false)))

(event EventControlTarget
  (params (Axis :type Vector%202D%20Structure) (ControlActor :type Actor%20Object%20Reference))
  (bind (_x _y) (Math|Vector2D|BreakVector2D Axis))
  (Class|PrimitiveComponent|AddAngularImpulseinRadians (Variables|Default|GetStaticMesh) (+ (* (Transformation|GetActorUpVector ControlActor) (* _y 8e+02 (.Y (Math|Vector|BreakVector (.location (Math|Transform|MakeRelativeTransform (Transformation|GetActorTransform) (Transformation|GetActorTransform ControlActor))))))) (* (Transformation|GetActorForwardVector ControlActor) (* _x (* (Math|Curves|GetFloatValue (Variables|Default|GetTouqueCurve_ControlStick) (CallFunction|WheelRotateSpeed)) -1.0 0.2)))) "None" false))

(event EventInteract
  (if (Variables|Default|GetON)
    (Variables|Default|SetON false)
    (else
      (Variables|Default|SetON true))))

(fn ConstructionScript
  (|CallParentFunction))

(fn WheelRotateSpeed
  (bind _staticmesh (Variables|Default|GetStaticMesh))
  (return (.X (Math|Vector|BreakVector (Math|Transform|InverseTransformDirection (Transformation|GetWorldTransform _staticmesh) (Physics|GetPhysicsAngularVelocityinDegrees _staticmesh "None"))))))