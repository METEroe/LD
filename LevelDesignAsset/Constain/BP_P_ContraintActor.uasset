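; BP_P_ContraintActor is a constraint-related actor that highlights under the mouse.
; It registers itself on BeginPlay.
; MouseOver and MouseEndOver toggle Render Custom Depth on its static mesh components through two DoOnce gates that reset each other, so each change fires once per hover transition.
; Request Interaction Info is a stub returning zero values, and the construction script is empty.
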(event EventBeginPlay
  (CallFunction|RegisterActor self))

(event EventMouseEndOver
  (Utilities|FlowControl|DoOnce false
    (:Completed
      (Rendering|SetRenderCustomDepth (Actor|GetComponentsByClass "/Script/Engine.StaticMeshComponent") false)
      (Utilities|FlowControl|DoOnce false) ; enters at Reset
    )))

(event EventMouseOver
  (Utilities|FlowControl|DoOnce false
    (:Completed
      (Rendering|SetRenderCustomDepth (Actor|GetComponentsByClass "/Script/Engine.StaticMeshComponent") true)
      (Utilities|FlowControl|DoOnce false) ; enters at Reset
    )))

(fn ConstructionScript)

(fn RequestInteractionInfo
  (return 0 0 0))