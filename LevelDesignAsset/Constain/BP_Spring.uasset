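; Spring level-design prop that draws a spline mesh stretched between two cubes, Cube and Cube1.
; Each tick and at construction, it sets the spline ends from the cubes' actor-relative transforms, with tangents along their forward vectors.
; An override event turns on physics for both cubes.
; It registers itself on BeginPlay, and mouse hover toggles custom depth highlighting through two DoOnce gates that reset each other.
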(event EventBeginPlay
  (CallFunction|RegisterActor self))

(event Collision|EventActorBeginOverlap
  (params (OtherActor :type Actor%20Object%20Reference)))

(event EventTick
  (params (DeltaSeconds :type Float%20%28single-precision%29))
  (CallFunction|UpdateSplineMesh))

(event EventMouseEndOver
  (Utilities|FlowControl|DoOnce false
    (:Completed
      (Rendering|SetRenderCustomDepth (Actor|GetComponentsByClass "/Script/Engine.StaticMeshComponent") false)
      (Utilities|FlowControl|DoOnce false) ; enters at Reset
    )))

(event EventCallTargetOverideSimulatePhysic
  (Physics|SetSimulatePhysics (Variables|Default|GetCube) true)
  (Physics|SetSimulatePhysics (Variables|Default|GetCube1) true))

(event EventMouseOver
  (Utilities|FlowControl|DoOnce false
    (:Completed
      (Rendering|SetRenderCustomDepth (Actor|GetComponentsByClass "/Script/Engine.StaticMeshComponent") true)
      (Utilities|FlowControl|DoOnce false) ; enters at Reset
    )))

(fn ConstructionScript
  (CallFunction|UpdateSplineMesh))

(fn UpdateSplineMesh
  (bind _returnvalue (Transformation|GetActorTransform))
  (bind _returnvalue_2 (Transformation|GetActorTransform))
  (bind _cube1 (Variables|Default|GetCube1))
  (bind _cube (Variables|Default|GetCube))
  (bind _splinemesh (Variables|Default|GetSplineMesh))
  (bind _returnvalue_3 (Transformation|GetWorldTransform _cube1))
  (bind _returnvalue_4 (Transformation|GetWorldTransform _cube))
  (bind _returnvalue_5 (Math|Transform|MakeRelativeTransform _returnvalue_4 _returnvalue_2))
  (bind _returnvalue_6 (Math|Transform|MakeRelativeTransform _returnvalue_3 _returnvalue))
  (SplineMesh|SetStartPosition _splinemesh (.location _returnvalue_5) false)
  (SplineMesh|SetEndPosition _splinemesh (.location _returnvalue_6) false)
  (SplineMesh|SetEndTangent _splinemesh (* (Math|Vector|GetForwardVector (.rotation _returnvalue_6)) 5e+02) false :!class /Script/Engine.SplineMeshComponent)
  (SplineMesh|SetStartTangent (Variables|Default|GetSplineMesh) (* (Math|Vector|GetForwardVector (.rotation _returnvalue_5)) 5e+02) true :!class /Script/Engine.SplineMeshComponent))

(fn RequestInteractionInfo
  (return 0 0 0))