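; BP_Gear_WithPower is a powered gear for physics-based level props that can be switched on and off.
; The Interact event toggles the ON flag.
; While ON and the static mesh is simulating physics, Tick applies a constant angular impulse along the mesh's up vector every frame to spin it, without scaling by delta time.
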(event EventBeginPlay
  (|CallParentFunction) ; This node is disabled and will not be called.\nDrag off pins to build functionality.
)

(event Collision|EventActorBeginOverlap
  (params (OtherActor :type Actor%20Object%20Reference))
  (|CallParentFunction OtherActor) ; This node is disabled and will not be called.\nDrag off pins to build functionality.
)

(event EventTick
  (params (DeltaSeconds :type Float%20%28single-precision%29))
  (bind _staticmesh (Variables|Default|GetStaticMesh))
  (|CallParentFunction DeltaSeconds)
  (if (and (Variables|Default|GetON) (Physics|IsSimulatingPhysics (Variables|Default|GetStaticMesh) "None"))
    (Class|PrimitiveComponent|AddAngularImpulseinRadians _staticmesh (* (Math|Vector|GetUpVector _staticmesh) 1e+05) "None" false)))

(event EventInteract
  (if (Variables|Default|GetON)
    (Variables|Default|SetON false)
    (else
      (Variables|Default|SetON true))))

(fn ConstructionScript
  (|CallParentFunction))