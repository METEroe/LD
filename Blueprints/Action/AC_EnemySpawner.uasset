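; AC_EnemySpawner is a timed action actor that triggers random enemy spawns while it lives.
; On BeginPlay it loops on a delay set by AC.Gap, calling NotifyRandomSpawnEnemyMessage on player controller 0 after each wait, so it does no spawning itself.
; A parallel delay set by AC.Duration destroys the actor, which ends the loop.
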(event EventBeginPlay
  (bind _ac (Variables|Default|GetAC))
  (bind (_displaytext _gap _duration) (Utilities|Struct|BreakS_AC _ac))
  (|CallParentFunction)
  (Utilities|FlowControl|Sequence
    (:then_0
      (Utilities|FlowControl|Delay _gap :!label _label)
      (Class|BPIController|NotifyRandomSpawnEnemy(Message) (Game|GetPlayerController 0))
      (goto _label))
    (:then_1
      (Utilities|FlowControl|Delay _duration)
      (Actor|DestroyActor))))

(event Collision|EventActorBeginOverlap
  (params (OtherActor :type Actor%20Object%20Reference)))

(event EventTick
  (params (DeltaSeconds :type Float%20%28single-precision%29)))

(fn ConstructionScript
  (|CallParentFunction))