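; AC_RunSequence is an action actor that plays a timed camera shot with on-screen text from its ActionData.
; On BeginPlay it applies the data's focus settings and world transform to its CineCamera, switches the player's view to itself, and sets its TextRender text.
; After the configured duration it notifies the player controller that the sequence ended, then destroys itself.
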(event EventBeginPlay
  (bind _action_data (Variables|Default|GetAction%20Data))
  (bind _cinecamera (Variables|Default|GetCineCamera))
  (bind _action_data_2 (Variables|Default|GetAction%20Data))
  (bind (_displaytext _gap _duration _type _classrefer _cameraworldtransform _camerafocussetting) (Utilities|Struct|BreakS_ActionInfo _action_data_2))
  (bind (_displaytext_2 _gap_2 _duration_2) (Utilities|Struct|BreakS_ActionInfo _action_data))
  (|CallParentFunction)
  (Variables|/Script/CinematicCamera.CineCameraComponent|SetFocusSettings _cinecamera _camerafocussetting)
  (Transformation|SetWorldTransform _cinecamera _cameraworldtransform false false)
  (Game|Player|SetViewTargetwithBlend (Game|GetPlayerController 0) self 0.0 "VTBlend_Linear" 0.0 false)
  (Rendering|Components|TextRender|SetText (Variables|Default|GetTextRender) (Utilities|Text|ToText(String) _displaytext_2))
  (Utilities|FlowControl|Delay _duration_2)
  (Class|BPIController|NotifySequenceEnd(Message) (Game|GetPlayerController 0))
  (Actor|DestroyActor))

(fn ConstructionScript
  (|CallParentFunction))