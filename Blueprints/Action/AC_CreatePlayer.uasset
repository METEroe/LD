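; AC_CreatePlayer is an action Blueprint that stages the player's arrival and level opening when it begins play.
; It has ChessController run the level, moves the pawn's capsule to the origin and spawns teleport, dot-up and spear Niagara effects.
; Between timed subtitles, it schedules enemy spawner actions on the controller, resets level time and clears enemies.
; A delayed loop then deals random cards from the hand pool before flagging the level as running.
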(event EventBeginPlay
  (|CallParentFunction)
  (Transformation|SetWorldLocation (Variables|Default|GetDefaultSceneRoot) "0.000000,0.000000,150.000000" false false)
  (bind _aschess_controller (Utilities|Casting|CastToChessController (Game|GetPlayerController 0)))
  (Variables|Default|SetAs%20Chess%20Controller _aschess_controller)
  (Default|RunLevel (Variables|Default|GetAs%20Chess%20Controller))
  (Transformation|SetWorldLocation (Variables|/Game/Blueprints/Character/BP_ControlPiece.BP_ControlPiece_C|GetCapsule (Variables|/Game/Blueprints/ChessController.ChessController_C|GetPlayer%20Pawn (Variables|Default|GetAs%20Chess%20Controller))) "0, 0, 0" false false)
  (Niagara|SpawnSystematLocation "/Game/VFX/NS_Teleport.NS_Teleport" "0, 0, 0")
  (Niagara|SpawnSystematLocation "/Game/VFX/NS_DotUp.NS_DotUp" "0, 0, 0")
  (Niagara|SpawnSystematLocation "/Game/VFX/NS_Spear.NS_Spear" "0, 0, 0")
  (Utilities|FlowControl|Delay 1.0)
  (Default|CallSubtitleShow (Variables|/Game/Blueprints/ChessController.ChessController_C|GetVirtual%20Desktop%20Widget (Variables|Default|GetAs%20Chess%20Controller)) "God! I can't believe you answer me.")
  (Variables|/Game/Blueprints/ChessController.ChessController_C|SetAction%20with%20Time (Variables|Default|GetAs%20Chess%20Controller) (Utilities|Array|MakeArray (Utilities|Struct|MakeS_ActionWithTime (Utilities|Struct|MakeS_AC "" 5.0 2e+01 0.0 "/Game/Blueprints/Action/AC_EnemySpawner.AC_EnemySpawner_C") 3.0) (Utilities|Struct|MakeS_ActionWithTime (Utilities|Struct|MakeS_AC "" 0.7 5.0 0.0 "/Game/Blueprints/Action/AC_EnemySpawner.AC_EnemySpawner_C") 2e+01)))
  (Variables|/Game/Blueprints/ChessController.ChessController_C|SetLevel%20Time (Variables|Default|GetAs%20Chess%20Controller) 0.0)
  (Default|ClearEnemy (Variables|Default|GetAs%20Chess%20Controller))
  (Utilities|FlowControl|Delay 4.5)
  (Default|CallSubtitleShow (Variables|/Game/Blueprints/ChessController.ChessController_C|GetVirtual%20Desktop%20Widget (Variables|Default|GetAs%20Chess%20Controller)) "Bring me their head. I can revive soldiers.")
  (Utilities|ForLoopwithDelay 0 3 0.5
    (:Loop%20Body
      (Default|CallControllerAddCard (Variables|Default|GetAs%20Chess%20Controller) (.OutItem (Utilities|Array|Random (Variables|/Game/Blueprints/ChessController.ChessController_C|GetPlayer%20Hand%20Cards%20Pool (Variables|Default|GetAs%20Chess%20Controller))))))
    (:Complete
      (Variables|/Game/Blueprints/ChessController.ChessController_C|SetLevel%20Is%20Runing (Variables|Default|GetAs%20Chess%20Controller) true))))

(fn ConstructionScript
  (|CallParentFunction))