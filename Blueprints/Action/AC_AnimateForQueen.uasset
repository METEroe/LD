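; AC_AnimateForQueen is a scripted action that plays a story beat about an unstoppable queen when it begins play.
; On BeginPlay it gets the ChessController from player 0, pauses the level and shows a subtitle hinting at a portal to the player's world.
; It then reveals the back-to-desktop button on the controller's virtual desktop widget.
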(event EventBeginPlay
  (|CallParentFunction)
  (bind _aschess_controller (Utilities|Casting|CastToChessController (Game|GetPlayerController 0)))
  (bind _output_get (Variables|Default|SetAs%20Chess%20Controller _aschess_controller))
  (Default|PauseLevel _output_get)
  (Class|BPIController|CallCreateSubtitle(Message) _output_get "This queen is too weird.  It is unstoppable. 
God, there is a portal link us to your world. Maybe you can find it.")
  (Variables|/Script/UMG.Widget|SetVisibility (Variables|/Game/Blueprints/WB_1_VirtualDesktop.WB_1_VirtualDesktop_C|GetButton_BackToDesktop (Variables|/Game/Blueprints/ChessController.ChessController_C|GetVirtual%20Desktop%20Widget _output_get)) "Visible"))

(event Collision|EventActorBeginOverlap
  (params (OtherActor :type Actor%20Object%20Reference)))

(event EventTick
  (params (DeltaSeconds :type Float%20%28single-precision%29)))

(fn ConstructionScript
  (|CallParentFunction))