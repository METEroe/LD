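; AC_FirstLevelEntry is the first level's intro cutscene actor, which becomes the player's view target through a camera blend on BeginPlay.
; Two timed Sequence branches set its text render to the King's lines and call StartTalk on the BP_KING actor.
; After the second line, a delayed loop sends repeated coin-get notifications to the ChessController, then signals that the sequence has ended.
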(event EventBeginPlay
  (|CallParentFunction)
  (bind _aschess_controller (Utilities|Casting|CastToChessController (Game|GetPlayerController 0)))
  (bind _output_get (Variables|Default|SetAs%20Chess%20Controller _aschess_controller))
  (Game|Player|SetViewTargetwithBlend _output_get self 1.5 "VTBlend_Linear" 0.0 false)
  (Utilities|FlowControl|Sequence
    (:then_0
      (Utilities|FlowControl|Delay 2.0)
      (Rendering|Components|TextRender|SetText (Variables|Default|GetTextRender) (Utilities|Text|MakeLiteralText "Die for me, my pawn 
Fight with enemy"))
      (bind _returnvalue (Actor|GetActorOfClass "/Game/Blueprints/Character/BP_KING.BP_KING_C"))
      (Default|StartTalk _returnvalue))
    (:then_1
      (Utilities|FlowControl|Delay 6.0)
      (Rendering|Components|TextRender|SetText (Variables|Default|GetTextRender) (Utilities|Text|MakeLiteralText "These are our only 
 remaining soldiers."))
      (bind _returnvalue_2 (Actor|GetActorOfClass "/Game/Blueprints/Character/BP_KING.BP_KING_C"))
      (Default|StartTalk _returnvalue_2)
      (Utilities|FlowControl|Delay 1.0)
      (Utilities|ForLoopwithDelay 0 3 0.3
        (:Loop%20Body
          (Class|BPIController|NotifyCoinGet(Message) (Variables|Default|GetAs%20Chess%20Controller)))
        (:Complete
          (Utilities|FlowControl|Delay 1.5)
          (Class|BPIController|NotifySequenceEnd(Message) (Variables|Default|GetAs%20Chess%20Controller)))))))

(fn ConstructionScript
  (|CallParentFunction))