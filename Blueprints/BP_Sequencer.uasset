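; BP_Sequencer is a one-shot scripted sequence actor that shifts the player's view to itself, reveals text and has the King talk.
; BeginPlay hides the TextRender and caches the ChessController and the BP_KING actor.
; CallSequenceBegin blends the view over, waits, shows the text and starts the King's talk.
; After a second fixed delay, it notifies the controller that the sequence has ended and destroys itself.
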(event Custom|Call%20Sequence%20Begin
  (Game|Player|SetViewTargetwithBlend (Variables|Default|GetChess%20COntroller) self 1.0 "VTBlend_Linear" 0.0 false)
  (Utilities|FlowControl|Delay 1.2)
  (Rendering|SetVisibility (Variables|Default|GetTextRender) true false)
  (Default|StartTalk (Variables|Default|GetKing))
  (Utilities|FlowControl|Delay 1.2)
  (Default|CallSequenceEnd (Variables|Default|GetChess%20COntroller))
  (Actor|DestroyActor))

(event EventBeginPlay
  (Rendering|SetVisibility (Variables|Default|GetTextRender) false false)
  (bind _aschess_controller (Utilities|Casting|CastToChessController (Game|GetPlayerController 0)))
  (Variables|Default|SetChess%20COntroller _aschess_controller)
  (bind _returnvalue (Actor|GetActorOfClass "/Game/Piece/BluePrints/BP_KING.BP_KING_C"))
  (Variables|Default|SetKing _returnvalue))

(fn ConstructionScript)