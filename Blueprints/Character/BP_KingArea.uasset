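; BP_KingArea is a resizable trigger volume that reports coin-get and player-death events to the ChessController.
; Shortly after BeginPlay it caches the ChessController and the BP_ControlPiece.
; When that piece overlaps with its pickup flag set, it plays a sound, notifies coin collection and clears the pickup flags.
; Any other overlapping actor triggers the player-death notification; the construction script sizes the box from InBoxExtent.
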(event OnComponentBeginOverlap(Box)
  (params (OverlappedComponent :type Primitive%20Component%20Object%20Reference) (OtherActor :type Actor%20Object%20Reference) (OtherComp :type Primitive%20Component%20Object%20Reference) (OtherBodyIndex :type Integer) (bFromSweep :type Boolean) (SweepResult :type Hit%20Result%20Structure%20%28by%20ref%29))
  (bind _as_bp_control_piece (Variables|Default|GetAs%20BP%20Control%20Piece))
  (if (== OtherActor (Variables|Default|GetAs%20BP%20Control%20Piece))
    (if (Variables|/Game/Blueprints/Character/BP_ControlPiece.BP_ControlPiece_C|GetPickUpFlag (Variables|Default|GetAs%20BP%20Control%20Piece))
      (Audio|PlaySound2D "/Game/SoundFX/Player/summon__stephensaldanha__magical_effect.summon__stephensaldanha__magical_effect" 1.0 1.0 0.0 0 0)
      (Class|BPIController|NotifyCoinGet(Message) (Variables|Default|GetAs%20Chess%20Controller))
      (Variables|/Game/Blueprints/Character/BP_ControlPiece.BP_ControlPiece_C|SetPickUpFlag _as_bp_control_piece false)
      (Variables|/Game/Blueprints/Character/BP_ControlPiece.BP_ControlPiece_C|SetAfter%20Pick _as_bp_control_piece false))
    (else
      (Class|BPIController|NotifyPlayerDie(Message) (Variables|Default|GetAs%20Chess%20Controller))
      (Development|PrintString "Fail"))))

(event EventBeginPlay
  (Utilities|FlowControl|Delay 0.2)
  (bind _aschess_controller (Utilities|Casting|CastToChessController (Game|GetPlayerController 0)))
  (Variables|Default|SetAs%20Chess%20Controller _aschess_controller)
  (bind _returnvalue (Actor|GetActorOfClass "/Game/Blueprints/Character/BP_ControlPiece.BP_ControlPiece_C"))
  (Variables|Default|SetAs%20BP%20Control%20Piece _returnvalue))

(fn ConstructionScript
  (Variables|Default|SetIn%20Box%20Extent (Variables|Default|GetIn%20Box%20Extent))
  (Components|Box|SetBoxExtent (Variables|Default|GetBox) (Variables|Default|GetIn%20Box%20Extent) true))