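; BP_ControlPiece is the player's piece: it moves on two axes, turns to face travel, and fights automatically in encounters.
; Encounter start enters a self-repeating attack loop of delayed BP_Bullet bursts with montage and sound, which does not recheck InGame.
; PickUpFlag reveals a mesh and adds a one-time pickup montage before attacking.
; Damage spawns text and shake, death notifies ChessController, and stats support save, load and reset.
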(event Custom|Xmove
  (params (NewParam :type Float%20%28double-precision%29))
  (Utilities|FlowControl|Sequence
    (:then_0
      (if (> NewParam 0.0)
        (Transformation|SetWorldRotation (Variables|Default|GetCapsule) "0.000000,180.000000,0.000000" false false)
        (elif (< NewParam 0.0)
          (Transformation|SetWorldRotation (Variables|Default|GetCapsule) "0, 0, 0" false false))))
    (:then_1
      (bind _output_get (Variables|Movement|SetX%20Location (Transformation|GetWorldLocation (Variables|Default|GetCapsule))))
      (Transformation|SetWorldLocation (Variables|Default|GetCapsule) (Math|Vector|MakeVector (.x _output_get) (+ (.y _output_get) (* NewParam (* (Variables|GrowData|GetSpeed) -1.0))) 0.0) false false)
      (if (== NewParam 0.0)
        (Variables|Default|SetXMove%20Flag false)
        (else
          (Variables|Default|SetXMove%20Flag true))))))

(event Custom|Ymove
  (params (NewParam :type Float%20%28double-precision%29))
  (Utilities|FlowControl|Sequence
    (:then_0
      (if (> NewParam 0.0)
        (Transformation|SetWorldRotation (Variables|Default|GetCapsule) "0.000000,-90.000000,0.000000" false false)
        (elif (< NewParam 0.0)
          (Transformation|SetWorldRotation (Variables|Default|GetCapsule) "0.000000,90.000000,0.000000" false false))))
    (:then_1
      (bind _output_get (Variables|Movement|SetY%20Location (Transformation|GetWorldLocation (Variables|Default|GetCapsule))))
      (Transformation|SetWorldLocation (Variables|Default|GetCapsule) (Math|Vector|MakeVector (+ (.x _output_get) (* NewParam (Variables|GrowData|GetSpeed))) (.y _output_get) 0.0) false false)
      (if (== NewParam 0.0)
        (Variables|Default|SetYMove%20Flag false)
        (else
          (Variables|Default|SetYMove%20Flag true))))))

(event Custom|Call%20Control%20Pawn%20Encounter%20Begin
  (bind _skeletalmesh (Variables|Default|GetSkeletalMesh))
  (bind _default_shoot_interval (Variables|GrowData|GetDefault%20Shoot%20Interval))
  (Variables|Default|SetIn%20game true)
  (if (Variables|Default|GetIn%20game)
    (if (Variables|Movement|GetPickUpFlag) :!label _label
      (if (Variables|Default|GetAfter%20Pick)
        (Utilities|FlowControl|Delay _default_shoot_interval :!label _label_2)
        (else
          (Animation|Montage|PlayMontage _skeletalmesh "/Game/Character/MainChar/Anim/Mainchar_pickup_Montage.Mainchar_pickup_Montage" 5.5
            (:OnCompleted
              (Variables|Default|SetAfter%20Pick true)))))
      (else
        (goto _label_2)))
    (Utilities|FlowControl|Sequence
      (:then_0
        (Utilities|ForLoopwithDelay 1 (Variables|GrowData|GetBullet%20Number) 0.1
          (:Loop%20Body
            (CallFunction|FireBullet))))
      (:then_1
        (Animation|Montage|PlayMontage _skeletalmesh "/Game/Character/MainChar/Anim/Mainchar_attack_Montage.Mainchar_attack_Montage" (/ 1.2 _default_shoot_interval)
          (:then
            (Utilities|FlowControl|Sequence
              (:then_0
                (goto _label))
              (:then_1
                (Utilities|FlowControl|Delay 1.0)
                (Audio|PlaySound2D "/Game/SoundFX/Player/attack_1__glaneur-de-sons__sword-swing-b-soft-05.attack_1__glaneur-de-sons__sword-swing-b-soft-05" 1.0 1.0 0.0 0 0)))))))))

(event Custom|Call%20Control%20Pawn%20Encounter%20End
  (Variables|Default|SetIn%20game false))

(event Custom|Load%20Game
  (params (Shoot%20Interval :type Float%20%28single-precision%29) (Damage :type Integer) (Speed :type Float%20%28double-precision%29) (Max%20Health :type Integer) (Bullet%20Number :type Integer) (Health :type Integer))
  (Variables|GrowData|SetShoot%20Interval Shoot%20Interval)
  (Variables|GrowData|SetDamage Damage)
  (Variables|GrowData|SetSpeed Speed)
  (Variables|GrowData|SetMax%20Health Max%20Health)
  (Variables|GrowData|SetBullet%20Number Bullet%20Number)
  (Variables|GrowData|SetHealth Health))

(event Custom|Fire%20Bullet
  (Game|SpawnActorfromClass "/Game/Blueprints/Character/BP_Bullet.BP_Bullet_C" (Transformation|GetWorldTransform (Variables|Default|GetArrow)) "Undefined" "MultiplyWithRoot" 0 (Variables|GrowData|GetBullet%20Speed) 0.0 1e+02 (Variables|GrowData|GetDamage) "NewEnumerator1" 0))

(event Custom|Clear%20Save
  (Variables|GrowData|SetShoot%20Interval (Variables|GrowData|GetDefault%20Shoot%20Interval))
  (Variables|GrowData|SetSpeed (Variables|GrowData|GetDefault%20Speed))
  (Variables|GrowData|SetDefault%20Damage (Variables|GrowData|GetDamage))
  (Variables|GrowData|SetMax%20Health (Variables|GrowData|GetDefault%20Max%20Health))
  (Variables|GrowData|SetBullet%20Number (Variables|GrowData|GetDefault%20Bullet%20Number))
  (Variables|GrowData|SetMax%20Health (Variables|GrowData|GetHealth)))

(event EventTick
  (params (DeltaSeconds :type Float%20%28single-precision%29))
  (if (Variables|Movement|GetPickUpFlag)
    (Development|SetHiddeninGame (Variables|Default|GetStaticMesh) false false)
    (else
      (Development|SetHiddeninGame (Variables|Default|GetStaticMesh) true false))))

(event EventBeginPlay)

(event EventApplyDamage
  (params (Damage :type Integer))
  ;[1 1 1] Health
  (Game|SpawnActorfromClass "/Game/Blueprints/Character/T_DamageText.T_DamageText_C" (Math|Transform|MakeTransform (+ (Transformation|GetWorldLocation (Variables|Default|GetCapsule)) "-80.000000,0.000000,40.000000") "0, 0, 0" "1.000000,1.000000,1.000000") "Undefined" "MultiplyWithRoot" 0 0 0)
  (Class|ShakerComponent|PlayShake (Variables|Default|GetShaker) "/Game/Blueprints/Character/Shake_Hit.Shake_Hit_C" 1.0)
  (bind _output_get (Variables|GrowData|SetHealth (- (Variables|GrowData|GetHealth) Damage)))
  (if (<= _output_get 0.0)
    (Audio|PlaySound2D "/Game/SoundFX/Death/death2_zmb94__pop5.death2_zmb94__pop5" 1.0 1.0 0.0 0 0)
    (Development|PrintString "Dead!")
    (Variables|GrowData|SetHealth 0)
    (Animation|Montage|PlayMontage (Variables|Default|GetSkeletalMesh) "/Game/Character/MainChar/Anim/Mainchar_pickup_Montage.Mainchar_pickup_Montage" 2.0
      (:OnCompleted
        (Class|BPIController|NotifyPlayerDie(Message) (Variables|Default|GetChessController))))
    (elif (> (Variables|GrowData|GetHealth) (Variables|GrowData|GetMax%20Health))
      (Variables|GrowData|SetMax%20Health (Variables|GrowData|GetMax%20Health)))))

(fn ConstructionScript)

(fn SaveGame
  (return (Variables|GrowData|GetShoot%20Interval) (Variables|GrowData|GetSpeed) (Variables|GrowData|GetHealth) (Variables|GrowData|GetMax%20Health) (Variables|GrowData|GetBullet%20Number) (Variables|GrowData|GetDamage)))

(fn RequestSlotData
  (return false "0, 0, 0"))