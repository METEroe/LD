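; Chess-piece pawn for both factions that fights automatically, with stats, mesh and anim class loaded from T_Chess by PawnType in the construction script.
; Player pieces always attack, while enemies advance along Y until a forward trace finds a player.
; A FireRate-scaled Timeline triggers per-type attacks: bullet patterns, or the Knight's self-destructing front-and-back trace strike.
; Damage spawns floating text and shake; death notifies the controller before destroying the piece.
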(event Custom|Make%20decision
  (switch Utilities|FlowControl|Switch|SwitchonE_ChessType (Variables|CommonData|GetPawn%20Type)))

(event Custom|Attack
  (if (Variables|CommonData|GetIn%20Attack%20Range)
    (Timeline|Timeline Play
      (:Archer_Attack
        (CallFunction|AttackDispatch)))))

(event Custom|Update%20Player%20Rate)

(event Custom|Attack%20Dispatch
  (bind _arrow (Variables|Default|GetArrow))
  (bind _skeletalmesh (Variables|Default|GetSkeletalMesh))
  (bind _arrow_2 (Variables|Default|GetArrow))
  (bind _capsule (Variables|Default|GetCapsule))
  (bind _capsule_2 (Variables|Default|GetCapsule))
  (bind _arrow_3 (Variables|Default|GetArrow))
  (bind _returnvalue (Transformation|GetWorldLocation _arrow))
  (bind _returnvalue_2 (Transformation|GetWorldLocation _arrow_3))
  (bind _returnvalue_3 (Transformation|GetWorldLocation _arrow_2))
  (bind _returnvalue_4 (Transformation|GetWorldLocation _capsule))
  (bind _returnvalue_5 (Transformation|GetWorldLocation _capsule_2))
  (switch Utilities|FlowControl|Switch|SwitchonE_ChessType (Variables|CommonData|GetPawn%20Type)
    (:NewEnumerator1
      (Niagara|SpawnSystematLocation 0 _returnvalue "0.000000,90.000000,0.000000")
      (Audio|PlaySoundatLocation 0 _returnvalue "0, 0, 0" 1.0 1.0 0.0 0 0 0 0)
      (Utilities|ForLoopwithDelay 0 3 0.2
        (:Loop%20Body
          (Audio|PlaySound2D "/Game/SoundFX/Player/attack_1__glaneur-de-sons__sword-swing-b-soft-05.attack_1__glaneur-de-sons__sword-swing-b-soft-05" 1.0 1.0 0.0 0 0)
          (Transformation|SetRelativeRotation (Variables|Default|GetArrow) (Math|Rotator|MakeRotator 0.0 0.0 (Math|Random|RandomFloatinRange -3e+01 3e+01)) false false)
          (CallFunction|FireBullet))))
    (:NewEnumerator5
      (Collision|SetCollisionEnabled _skeletalmesh "NoCollision")
      (Utilities|FlowControl|Sequence
        (:then_0
          (Utilities|FlowControl|Sequence
            (:then_0
              (Utilities|FlowControl|Delay 1.0)
              (Actor|DestroyActor))
            (:then_1
              (bind _outhits (Collision|MultiLineTraceByChannel (+ (* (Math|Vector|GetForwardVector (Transformation|GetWorldRotation _capsule_2)) 2.5e+02) _returnvalue_5) (+ _returnvalue_5 (* (Math|Vector|GetForwardVector (Transformation|GetWorldRotation _capsule_2)) 1e+03)) "TraceTypeQuery1" false 0 "ForOneFrame"))
              (for _array_element _outhits
                (Development|PrintString (Utilities|GetDisplayName (.HitActor (Collision|BreakHitResult _array_element))))
                (Class|BPIInteraction|ApplyDamage(Message) (.HitActor (Collision|BreakHitResult _array_element)) (Math|Float|Truncate (Variables|Default|GetDamage)))))
            (:then_2
              (bind _outhits_2 (Collision|MultiLineTraceByChannel (+ (* (Math|Vector|GetForwardVector (Transformation|GetWorldRotation _capsule)) -2.5e+02) _returnvalue_4) (+ _returnvalue_4 (* (Math|Vector|GetForwardVector (Transformation|GetWorldRotation _capsule)) -1e+03)) "TraceTypeQuery1" false 0 "ForOneFrame"))
              (for _array_element_2 _outhits_2
                (Class|BPIInteraction|ApplyDamage(Message) (.HitActor (Collision|BreakHitResult _array_element_2)) (Math|Float|Truncate (Variables|Default|GetDamage)))))
            (:then_3
              (Audio|PlaySound2D "/Game/SoundFX/Player/downward_smash_knight__15gkovacovajulie__110_burning-paper.downward_smash_knight__15gkovacovajulie__110_burning-paper" 1.0 1.0 0.0 0 0))))
        (:then_1
          (Animation|Montage|PlayMontage _skeletalmesh "/Game/Character/Ally/SKM_Knight_Anim_Montage.SKM_Knight_Anim_Montage"))))
    (:NewEnumerator2
      (Niagara|SpawnSystematLocation 0 (Transformation|GetWorldLocation (Variables|Default|GetArrow)) "0.000000,90.000000,0.000000")
      (bind _index (Utilities|ForLoopwithDelay 0 3 0.0)
        (:Loop%20Body
          (Audio|PlaySound2D "/Game/SoundFX/Player/attack_1__glaneur-de-sons__sword-swing-b-soft-05.attack_1__glaneur-de-sons__sword-swing-b-soft-05" 1.0 1.0 0.0 0 0)
          (Transformation|SetRelativeRotation (Variables|Default|GetArrow) (Math|Rotator|MakeRotator 0.0 0.0 (Math|Conversions|ToFloat(Integer) (+ (* _index 90) 45))) false false)
          (CallFunction|FireBullet))))
    (:NewEnumerator3
      (Niagara|SpawnSystematLocation 0 _returnvalue_2 "0.000000,90.000000,0.000000")
      (Audio|PlaySoundatLocation 0 _returnvalue_2 "0, 0, 0" 1.0 1.0 0.0 0 0 0 0)
      (Audio|PlaySound2D "/Game/SoundFX/Player/attack_1__glaneur-de-sons__sword-swing-b-soft-05.attack_1__glaneur-de-sons__sword-swing-b-soft-05" 1.0 1.0 0.0 0 0)
      (CallFunction|FireBullet))
    (:NewEnumerator4
      (Niagara|SpawnSystematLocation 0 _returnvalue_3 "0.000000,90.000000,0.000000" :!label _label)
      (Audio|PlaySoundatLocation 0 _returnvalue_3 "0, 0, 0" 1.0 1.0 0.0 0 0 0 0)
      (Audio|PlaySound2D "/Game/SoundFX/Player/attack_1__glaneur-de-sons__sword-swing-b-soft-05.attack_1__glaneur-de-sons__sword-swing-b-soft-05" 1.0 1.0 0.0 0 0)
      (CallFunction|FireBullet))
    (:NewEnumerator6
      (goto _label))
    (:NewEnumerator7
      (goto _label))
    (:NewEnumerator8
      (goto _label))))

(event Custom|Fire%20Bullet
  (Game|SpawnActorfromClass "/Game/Blueprints/Character/BP_Bullet.BP_Bullet_C" (Transformation|GetWorldTransform (Variables|Default|GetArrow)) "Undefined" "MultiplyWithRoot" 0 (Variables|Default|GetInitial%20Speed) (Variables|Default|GetPawn%20Speed) (Variables|Default|GetLife%20Span) (Math|Float|Truncate (Variables|Default|GetDamage)) (Variables|CommonData|GetHit%20Target%20Actor) 0))

(event EventTick
  (params (DeltaSeconds :type Float%20%28single-precision%29))
  (bind _capsule (Variables|Default|GetCapsule))
  (bind _returnvalue (Transformation|GetWorldLocation _capsule))
  (CallFunction|MakeDecision)
  (CallFunction|Attack)
  (if (Variables|CommonData|GetIs%20Enemy)
    (Utilities|FlowControl|Sequence
      (:then_0
        (bind (_outhit _returnvalue_2) (Collision|LineTraceForObjects _returnvalue (+ _returnvalue (* (Math|Vector|GetForwardVector (Transformation|GetWorldRotation _capsule)) 7e+01)) (Utilities|Array|MakeArray "ObjectTypeQuery3") false 0 "None"))
        (if _returnvalue_2
          (Variables|CommonData|SetIn%20Attack%20Range (Actor|ActorHasTag (.HitActor (Collision|BreakHitResult _outhit)) "Player"))
          (else
            (Variables|CommonData|SetIn%20Attack%20Range false))))
      (:then_1
        (if (Variables|CommonData|GetIn%20Attack%20Range)
          (CallFunction|Attack)
          (else
            (Transformation|SetWorldLocation (Variables|Default|GetCapsule) (+ (Transformation|GetWorldLocation (Variables|Default|GetCapsule)) (Math|Vector|MakeVector 0.0 (* (* (+ (Variables|Default|GetPawn%20Speed) 1.0) (Variables|CommonData|GetEnemy%20Speed)) (Utilities|Time|GetWorldDeltaSeconds)) 0.0)) false false)))))))

(event EventBeginPlay
  (if (Variables|CommonData|GetIs%20Enemy)
    (Transformation|SetWorldRotation (Variables|Default|GetCapsule self) "0.000000,-90.000000,0.000000" false false)
    (else
      (Transformation|SetWorldRotation (Variables|Default|GetCapsule self) "0.000000,90.000000,0.000000" false false))))

(event EventApplyDamage
  (params (Damage :type Integer))
  ;[1 1 1] Health
  (Game|SpawnActorfromClass "/Game/Blueprints/Character/T_DamageText.T_DamageText_C" (Math|Transform|MakeTransform (+ (Transformation|GetWorldLocation (Variables|Default|GetCapsule)) "-80.000000,0.000000,40.000000") "0, 0, 0" "1.000000,1.000000,1.000000") "Undefined" "MultiplyWithRoot" 0 Damage 0)
  (Class|ShakerComponent|PlayShake (Variables|Default|GetShaker) "/Game/Blueprints/Character/Shake_Hit.Shake_Hit_C" 1.0)
  (bind _output_get (Variables|Health|SetHealth (- (Variables|Health|GetHealth) Damage)))
  (if (<= _output_get 0.0)
    (Audio|PlaySound2D "/Game/SoundFX/Death/death2_zmb94__pop5.death2_zmb94__pop5" 1.0 1.0 0.0 0 0)
    (Variables|Health|SetHealth 0.0)
    (if (Variables|CommonData|GetIs%20Enemy)
      (Class|BPIController|NotifyEnemyPieceDestory(Message) (Variables|Default|GetControlller%20refer) self)
      (else
        (Class|BPIController|NotifyPlayerPieceDestory(Message) (Variables|Default|GetControlller%20refer) self)))
    (Utilities|FlowControl|DelayUntilNextTick)
    (Actor|DestroyActor)
    (elif (> (Variables|Health|GetHealth) (Variables|Health|GetMax_Health))
      (Variables|Health|SetHealth (Variables|Health|GetMax_Health)))))

(fn ConstructionScript
  (bind _returnvalue (Utilities|GetDataTableRow "/Game/Blueprints/T_Chess.T_Chess" (Utilities|String|StringToName (Utilities|String|EnumtoString (Variables|CommonData|GetPawn%20Type))))
    (:then
      (Variables|Default|SetInitial%20Speed (.InitialSpeed (Utilities|Struct|BreakS_ChessData _returnvalue)))
      (Variables|Health|SetMax_Health (.MaxHealth (Utilities|Struct|BreakS_ChessData _returnvalue)))
      (Variables|Health|SetHealth (.Health (Utilities|Struct|BreakS_ChessData _returnvalue)))
      (Variables|Default|SetLife%20Span (.LifeSpan (Utilities|Struct|BreakS_ChessData _returnvalue)))
      (Variables|Default|SetDamage (.Damage (Utilities|Struct|BreakS_ChessData _returnvalue)))
      (Variables|Default|SetPawn%20Speed (.PawnSpeed (Utilities|Struct|BreakS_ChessData _returnvalue)))
      (Variables|Default|SetFire%20Rate (.Firerate (Utilities|Struct|BreakS_ChessData _returnvalue)))
      (Components|Timeline|SetPlayRate (Variables|Default|GetTimeline) (Variables|Default|GetFire%20Rate))
      (Components|SkeletalMesh|SetSkeletalMeshAsset (Variables|Default|GetSkeletalMesh) (.Mesh (Utilities|Struct|BreakS_ChessData _returnvalue)))
      (Utilities|Array|Add (Variables|Actor|GetTags) (Utilities|String|StringToName (Utilities|String|EnumtoString (Variables|CommonData|GetFaction%20Tag))))
      (Class|SkeletalMeshComponent|SetAnimClass (Variables|Default|GetSkeletalMesh) (.ABP (Utilities|Struct|BreakS_ChessData _returnvalue)))
      (switch Utilities|FlowControl|Switch|SwitchonE_Faction (Variables|CommonData|GetFaction%20Tag)
        (:NewEnumerator0
          (Variables|CommonData|SetHit%20Target%20Actor "NewEnumerator1")
          (Variables|CommonData|SetIn%20Attack%20Range true))
        (:NewEnumerator1
          (Variables|CommonData|SetHit%20Target%20Actor "NewEnumerator0")
          (Variables|CommonData|SetIs%20Enemy true))))))

(fn RequestSlotData
  (return false "0, 0, 0"))