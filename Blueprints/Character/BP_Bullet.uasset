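; BP_Bullet is a projectile actor that damages actors carrying a configurable target tag.
; The construction script applies its variables for initial speed, gravity scale and lifespan.
; On sphere overlap, it converts the HitTargetTag enum to a name, matches it against the other actor's tags and sends BaseDamage through ApplyDamageMessage.
; A matching hit then triggers PlayDMG, which spawns impact sounds and effects before destroying the bullet.
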(event OnComponentBeginOverlap(Sphere)
  (params (OverlappedComponent :type Primitive%20Component%20Object%20Reference) (OtherActor :type Actor%20Object%20Reference) (OtherComp :type Primitive%20Component%20Object%20Reference) (OtherBodyIndex :type Integer) (bFromSweep :type Boolean) (SweepResult :type Hit%20Result%20Structure%20%28by%20ref%29))
  (if (Utilities|Array|ContainsItem (Variables|/Script/Engine.Actor|GetTags OtherActor) (Utilities|String|StringToName (Utilities|String|EnumtoString (Variables|Default|GetHit%20Target%20Tag))))
    (Class|BPIInteraction|ApplyDamage(Message) OtherActor (Variables|Default|GetBase%20Damage))
    (CallFunction|PlayDMG)))

(event Custom|PlayDMG
  (bind _staticmesh (Variables|Default|GetStaticMesh))
  (bind _returnvalue (Transformation|GetWorldLocation _staticmesh))
  (Audio|PlaySoundatLocation 0 _returnvalue "0, 0, 0" 1.0 1.0 0.0 0 0 0 0)
  (Niagara|SpawnSystematLocation 0 _returnvalue "0.000000,0.000000,-90.000000" "0.200000,0.200000,0.200000")
  (Niagara|SpawnSystematLocation 0 _returnvalue "0.000000,90.000000,0.000000")
  (Audio|PlaySoundatLocation "/Game/SoundFX/Player/hitting__adhdreaming__rides-here-kick.hitting__adhdreaming__rides-here-kick" _returnvalue "0, 0, 0" 1.0 1.0 0.0 0 0 0 0)
  (Actor|DestroyActor))

(fn ConstructionScript
  (Variables|/Script/Engine.ProjectileMovementComponent|SetInitialSpeed (Variables|Default|GetProjectileMovement) (Variables|Default|GetInitial%20Speed))
  (Variables|/Script/Engine.ProjectileMovementComponent|SetProjectileGravityScale (Variables|Default|GetProjectileMovement) (Variables|Default|GetProjectile%20Gravity%20Scale))
  (Actor|SetLifeSpan (Variables|Default|GetIn%20Lifespan)))