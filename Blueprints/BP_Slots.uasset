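; BP_Slots is a grid slot tile that shows an index label and reports whether it is filled.
; The construction script scales the tile and highlight from Size, writes Index to the text, and picks a black or white grid material from Is1.
; MouseOver and MouseEndOver events show and hide the LightRayCube highlight.
; RequestSlotData returns IsFill and a world position 200 units above the slot's root.
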(event EventMouseOver
  (Rendering|SetVisibility (Variables|Default|GetLightRayCube) true false))

(event EventMouseEndOver
  (Rendering|SetVisibility (Variables|Default|GetLightRayCube) false false))

(fn ConstructionScript
  (bind _size (Variables|Default|Getsize))
  (bind _returnvalue (/ _size 1e+02))
  (bind _returnvalue_2 (- _size 5.0))
  (bind _returnvalue_3 (/ _returnvalue_2 2.0))
  (Transformation|SetRelativeScale3D (Variables|Default|GetLightRayCube) (Math|Vector|MakeVector _returnvalue_3 _returnvalue_3 _returnvalue_3))
  (Transformation|SetRelativeScale3D (Variables|Default|GetCube) (Math|Vector|MakeVector _returnvalue _returnvalue 1.0))
  (Rendering|Components|TextRender|SetText (Variables|Default|GetTextRender) (Utilities|Text|ToText(Integer) (Variables|Default|Getindex)))
  (if (Variables|Default|Getis%201)
    (Rendering|Material|SetMaterial (Variables|Default|GetCube) 0 "/Game/Blueprints/AssetData/BasicMaterial/M_GridBlack.M_GridBlack")
    (else
      (Rendering|Material|SetMaterial (Variables|Default|GetCube) 0 "/Game/Blueprints/AssetData/BasicMaterial/M_GridWhite.M_GridWhite"))))

(fn RequestSlotData
  (return (Variables|Default|GetIs%20Fill) (+ (Transformation|GetWorldLocation (Variables|Default|GetDefaultSceneRoot)) "0.000000,0.000000,200.000000")))