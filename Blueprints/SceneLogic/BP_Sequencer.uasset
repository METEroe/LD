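; BP_Sequencer is a one-shot scripted scene actor that moves the player's view to itself while the King talks.
; On BeginPlay it hides its text render and caches the BP_KING actor.
; CallSequenceBegin blends the camera to this actor, waits, reveals the text and starts the King's talk.
; After a second delay it notifies the player controller that the sequence has ended, then destroys itself.
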(event Custom|Call%20Sequence%20Begin
  (Game|Player|SetViewTargetwithBlend (Game|GetPlayerController 0) self 1.0 "VTBlend_Cubic" 0.0 false)
  (Utilities|FlowControl|Delay (Variables|Default|GetDelay%20Before%20Talk))
  (Rendering|SetVisibility (Variables|Default|GetTextRender) true false)
  (Default|StartTalk (Variables|Default|GetKing))
  (Utilities|FlowControl|Delay (Variables|Default|GetDelay%20after%20talk))
  (Class|BPIController|NotifySequenceEnd(Message) (Game|GetPlayerController 0))
  (Actor|DestroyActor))

(event EventBeginPlay
  (Rendering|SetVisibility (Variables|Default|GetTextRender) false false)
  (bind _returnvalue (Actor|GetActorOfClass "/Game/Blueprints/Character/BP_KING.BP_KING_C"))
  (Variables|Default|SetKing _returnvalue))

(fn ConstructionScript)