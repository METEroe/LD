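; BP_GameTable is a board actor for a chess-style game that builds a Row by Column grid of BP_Slots.
; The construction script scales and centers the Cube to the grid, and records a spawn point with an arrow marker just past one edge for each row.
; BeginPlay spawns and attaches the indexed slots, offsets the spawn points by the root's world location, and reports them to the ChessController.
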(event EventBeginPlay
  (bind _spawn_location (Variables|Default|GetSpawn%20Location))
  (for _index (range 0 (- (Variables|Default|GetRow) 1))
    (for _index_2 (range 0 (- (Variables|Default|GetColumn) 1))
      (bind _returnvalue (Game|SpawnActorfromClass "/Game/Controller/BP_Slots.BP_Slots_C" (Math|Transform|MakeTransform (Math|Vector|MakeVector (* _index (Variables|Default|GetSize)) (* _index_2 (Variables|Default|GetSize)) 0.0) "0, 0, 0" "1.000000,1.000000,1.000000") "Undefined" "MultiplyWithRoot" 0 (Variables|Default|GetSize) (+ (* _index (Variables|Default|GetRow)) _index_2) 0))
      (Transformation|AttachActorToActor _returnvalue self "None" "KeepRelative" "KeepRelative" "KeepRelative" true)))
  (bind _aschess_controller (Utilities|Casting|CastToChessController (Game|GetPlayerController 0)))
  (Variables|Default|Set%20Chess%20Controller _aschess_controller)
  (for (_array_element _array_index) _spawn_location
    (Utilities|Array|SetArrayElem _spawn_location _array_index (+ _array_element (Transformation|GetWorldLocation (Variables|Default|GetDefaultSceneRoot)))))
  (Default|ReportTableLoad (Variables|Default|Get%20Chess%20Controller) (Variables|Default|GetSpawn%20Location)))

(fn ConstructionScript
  (bind _size (Variables|Default|GetSize))
  (bind _column (Variables|Default|GetColumn))
  (bind _size_2 (Variables|Default|GetSize))
  (bind _returnvalue (/ _size_2 2.0))
  (bind _returnvalue_2 (* _size _column))
  (Transformation|SetRelativeScale3D (Variables|Default|GetCube) (Math|Vector|MakeVector (* (Math|Conversions|ToFloat(Integer) (Variables|Default|GetRow)) (/ (Variables|Default|GetSize) 1e+02)) (* (Math|Conversions|ToFloat(Integer) (Variables|Default|GetColumn)) (/ (Variables|Default|GetSize) 1e+02)) 1.0))
  (Transformation|SetRelativeLocation (Variables|Default|GetCube) (Math|Vector|MakeVector (- (/ (* (Math|Conversions|ToFloat(Integer) (Variables|Default|GetRow)) _size_2) 2.0) _returnvalue) (- (/ (* (Math|Conversions|ToFloat(Integer) (Variables|Default|GetColumn)) (Variables|Default|GetSize)) 2.0) _returnvalue) 0.0) false false)
  (for _index (range 0 (- (Variables|Default|GetRow) 1))
    (bind _returnvalue_3 (AddComponent|AddArrowComponent false (Math|Transform|MakeTransform (Math|Vector|MakeVector (* (Variables|Default|GetSize) _index) _returnvalue_2 0.0) "0.000000,-90.000000,0.000000" "1.000000,1.000000,1.000000")))
    (Variables|/Script/Engine.ArrowComponent|SetArrowSize _returnvalue_3 2e+01)
    (Variables|/Script/Engine.ArrowComponent|SetArrowLength _returnvalue_3 1e+01)
    (Utilities|Array|Add (Variables|Default|GetSpawn%20Location) (Math|Vector|MakeVector (* (Variables|Default|GetSize) _index) _returnvalue_2 0.0))))