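; BP_P_Interact is an interactable actor that toggles a hover highlight, with its interaction logic left as stubs.
; Construction sets custom depth stencil 1 on its static meshes for a post-process style highlight.
; MouseOver and MouseEndOver switch custom depth rendering on and off through two DoOnce gates that reset each other, so each change fires once per hover transition.
; InteracttoTarget is empty and Request Interaction Info returns zeros.
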(event EventBeginPlay)

(event Collision|EventActorBeginOverlap
  (params (OtherActor :type Actor%20Object%20Reference)))

(event EventTick
  (params (DeltaSeconds :type Float%20%28single-precision%29)))

(event EventMouseEndOver
  (Utilities|FlowControl|DoOnce false
    (:Completed
      (Rendering|SetRenderCustomDepth (Actor|GetComponentsByClass "/Script/Engine.StaticMeshComponent") false)
      (Utilities|FlowControl|DoOnce false) ; enters at Reset
    )))

(event EventMouseOver
  (Utilities|FlowControl|DoOnce false
    (:Completed
      (Rendering|SetRenderCustomDepth (Actor|GetComponentsByClass "/Script/Engine.StaticMeshComponent") true)
      (Utilities|FlowControl|DoOnce false) ; enters at Reset
    )))

(event EventInteracttoTarget
  (params (Input%20Type :type E_InteractType%20Enum :default "NewEnumerator0")))

(fn ConstructionScript
  (Rendering|SetCustomDepthStencilValue (Actor|GetComponentsByClass "/Script/Engine.StaticMeshComponent") 1))

(fn RequestInteractionInfo
  (return 0 0 0))